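; BP_River is a placeable river water actor with editable colors, opacity and depth settings.
; Its construction script creates a dynamic instance of WaterMaterial on slot 0 of the static mesh, then pushes those variables into the material's parameters.
; It has no runtime logic, and a node to set Water Height from the mesh's world Z is present but never runs.
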(fn `UserConstructionScript`
  (bind _returnvalue (`PrimitiveComponent.CreateDynamicMaterialInstance` (`self.StaticMeshComponent`) 0 (`self.Water Material`) "None"))
  (bind _output_get (set `self.Dynamic Material` _returnvalue))
  (`MaterialInstanceDynamic.SetVectorParameterValue` _output_get "WaterColor A" (`self.Primary Water Color`))
  (`MaterialInstanceDynamic.SetVectorParameterValue` _output_get "WaterColor B" (`self.Secondary Water Color`))
  (`MaterialInstanceDynamic.SetScalarParameterValue` _output_get "Base Opacity" (`self.Base Opacity`))
  (`MaterialInstanceDynamic.SetScalarParameterValue` _output_get "Shore Depth" (`self.Shore Depth`))
  (`MaterialInstanceDynamic.SetScalarParameterValue` _output_get "Water Depth" (`self.Water Depth`))
  (`MaterialInstanceDynamic.SetVectorParameterValue` _output_get "DeepWater" (`self.Deep Water Color`))
  (`MaterialInstanceDynamic.SetVectorParameterValue` _output_get "ShallowWater" (`self.Shallow Water Color`)))