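; Base Blueprint for an AI crewmember character in the ant crew, providing ability and death events.
; UseAbility switches on the ability number, but no branch has any logic, and the captain target data is unused.
; Die runs the parent logic, tells the controller its character died, then starts a delay that leads nowhere, leaving the DestroyActor node unreachable.
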(event `UseAbility`
  (params (AbilityNumber :type Integer) (CaptainTargetData :type "HitResult Structure"))
  (switch `int` AbilityNumber))

(event `self.Die`
  (`parent.Die`)
  (message `/Game/BPs/Interfaces/AiControllerCommunicationInterface.ControlledCharacterDied` (`self.GetController`))
  (`KismetSystemLibrary.Delay` 20.0))

(fn `UserConstructionScript`
  (`parent.UserConstructionScript`))