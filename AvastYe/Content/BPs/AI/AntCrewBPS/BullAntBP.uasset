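; Bull ant AI Blueprint, apparently an ant crew member, with a charge attack that rams and launches non-allies.
; CombatCharge raises walk speed and moves to a snapshot of the target's location; Tick stops movement and restores speed on arrival.
; While charging, sphere overlaps send a damage message with knockback and hit stun, skipping the captain and crew.
; BeginCharge and EndCharge also toggle the charge state independently of targeting.
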(event `self.ReceiveTick`
  (params (DeltaSeconds :type "Float (single-precision)"))
  (`parent.ReceiveTick` DeltaSeconds)
  (if (`self.IsUsingChargeAbiliy`)
    (if (<= (`KismetMathLibrary.VSize` (- (`self.ChargeLocation`) (`self.K2_GetActorLocation`))) 100.0)
      (`Controller.StopMovement` (`AIBlueprintHelperLibrary.GetAIController` self))
      (set `self.IsUsingChargeAbiliy` false)
      (`self.EndCharge`))))

(event `BeginCharge`
  (set `CharacterMovementComponent.MaxWalkSpeed` (`self.ChargeSpeed`) (`self.CharacterMovement`))
  (set `self.IsCharging` true))

(event `EndCharge`
  (set `CharacterMovementComponent.MaxWalkSpeed` (`self.WalkSpeed`) (`self.CharacterMovement`))
  (set `self.IsCharging` false))

(event `CombatCharge`
  (params (TargetEnemy :type "Actor Object Reference"))
  (bind _returnvalue (`self.K2_GetActorLocation` TargetEnemy))
  (set `CharacterMovementComponent.MaxWalkSpeed` (`self.ChargeSpeed`) (`self.CharacterMovement`))
  (set `self.IsCharging` true)
  (`NavigationSystem.SimpleMoveToLocation` (`AIBlueprintHelperLibrary.GetAIController` self) _returnvalue)
  (set `self.IsUsingChargeAbiliy` true)
  (set `self.ChargeLocation` _returnvalue))

(event `self.Sphere.OnComponentBeginOverlap`
  (params (OverlappedComponent :type "PrimitiveComponent Object Reference") (OtherActor :type "Actor Object Reference") (OtherComp :type "PrimitiveComponent Object Reference") (OtherBodyIndex :type Integer) (bFromSweep :type Boolean) (SweepResult :type "HitResult Structure (by ref)"))
  (bind _returnvalue (`GameplayStatics.GetObjectClass` OtherActor))
  (if (`self.IsCharging`)
    (if (not (or (== _returnvalue "/Game/BPs/CaptainCharacterBP.CaptainCharacterBP_C") (`KismetMathLibrary.ClassIsChildOf` _returnvalue "/Game/BPs/AI/AntCrewBPS/BaseCrewmemberAIBP.BaseCrewmemberAIBP_C")))
      (message `/Game/BPs/DamagableInterface.getDamaged` OtherActor 20.0 "NewEnumerator3" "none" (100.0 100.0 700.0) 1.0))))

(fn `UserConstructionScript`
  (`parent.UserConstructionScript`))