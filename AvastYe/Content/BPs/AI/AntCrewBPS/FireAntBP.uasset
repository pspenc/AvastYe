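; Fire ant Blueprint in the ant crew that throws fire at flammable interactable objects.
; ThrowFire casts the target to InteractableObject, turns the ant on yaw only toward its InteractPoint, then spawns a FireAntProjectile from the ant's location along the full look-at rotation, with itself as instigator.
; The event graph holds only disabled default events, and nothing in this file calls ThrowFire.
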(fn `Throw Fire`
  (params (`Flammable Object` :type "Actor Object Reference"))
  (bind _returnvalue (`self.K2_GetActorLocation` self))
  (bind _asinteractable_object (cast `/Game/BPs/PuzzleInteractables/InteractableObject` `Flammable Object`))
  (bind _returnvalue_2 (`KismetMathLibrary.FindLookAtRotation` _returnvalue (`SceneComponent.K2_GetComponentLocation` (`/Game/BPs/PuzzleInteractables/InteractableObject.InteractPoint` _asinteractable_object))))
  (`self.K2_SetActorRotation` (`KismetMathLibrary.MakeRotator` 0.0 0.0 (.yaw _returnvalue_2)))
  (`|SpawnActorFromClass` "/Game/BPs/FireAntProjectile.FireAntProjectile_C" (`KismetMathLibrary.MakeTransform` _returnvalue _returnvalue_2) "AlwaysSpawn" "OverrideRootScale" null self))

(fn `UserConstructionScript`
  (`parent.UserConstructionScript`))