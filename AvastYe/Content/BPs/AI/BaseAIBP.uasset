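; Base AI character Blueprint that extends a parent's damage and death handling and relays death, death reactions and ability completion to its controller.
; Taking damage from a CaptainCharacter occasionally rewards that attacker with ammo, and death optionally destroys the actor.
; Ability 0 is a sphere-trace AoE blast that damages and launches hits upward.
; Helpers aim projectile transforms at the blackboard target and cycle waypoints by bitmask, which wraps correctly only for power-of-two counts.
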(event `/Game/BPs/Interfaces/DamagableInterface.getDamaged`
  (params (DamageDealt :type "Float (single-precision)") (DamageType :type "/Game/BPs/GlobalEnums/DamageTypes Enum" :default "NewEnumerator0") (EnemyTeamTag :type "GameplayTag Structure") (ForceVector :type "Vector Structure") (HitStun :type "Float (single-precision)") (Attacker :type "/Game/BPs/BaseCharacterBP Object Reference") (HitComponent :type "PrimitiveComponent Object Reference"))
  (`parent.getDamaged` DamageDealt DamageType EnemyTeamTag ForceVector HitStun Attacker null)
  (bind _ascaptain_character (cast `/Game/BPs/CaptainCharacter` Attacker))
  (if (< (`KismetMathLibrary.RandomInteger` 10) 1)
    (`/Game/BPs/CaptainCharacter.AddAmmo` _ascaptain_character (`KismetMathLibrary.RandomIntegerInRange` 0 (`KismetMathLibrary.FTrunc` DamageDealt)))))

(event `self.Die`
  (`parent.Die`)
  (message `/Game/BPs/Interfaces/AICommunicationInterface.ControlledCharacterDied` (`self.GetController`))
  (if (`self.Do I Get Thanosed When I Die`)
    (`self.K2_DestroyActor`)))

(event `ReactToDeath`
  (params (KilledCharacter :type "/Game/BPs/BaseCharacterBP Object Reference"))
  (message `/Game/BPs/Interfaces/AICommunicationInterface.ReactToDeath` (`self.GetController`) KilledCharacter))

(event `Ability`
  (params (AbilityNumber :type Integer))
  (switch `int` AbilityNumber
    (:`0`
      (`self.AoeBoom`))))

(event `AoeBoom`
  (bind _returnvalue (`self.K2_GetActorLocation`))
  (bind _outhits (`KismetSystemLibrary.SphereTraceMultiForObjects` :`Start` _returnvalue :`End` _returnvalue :`Radius` 200.0 :`ObjectTypes` (`|MakeArray` "ObjectTypeQuery7" "ObjectTypeQuery8" :!type "EObjectTypeQuery Enum") :`DrawDebugType` "ForDuration" :`DrawTime` 1.0))
  (for _array_element _outhits
    (message `/Game/BPs/Interfaces/DamagableInterface.getDamaged` (`.HitActor` (`GameplayStatics.BreakHitResult` _array_element)) 30.0 "NewEnumerator0" (`self.EnemyTeamTag`) (0.0 0.0 520.0) 0.0 null null))
  (message `/Game/BPs/Interfaces/AICommunicationInterface.FinishAbility` (`self.GetController`)))

(event `ReturnNextWaypoint`
  (bind _result (`/Engine/EditorBlueprintResources/StandardMacros.IncrementInt` (`self.CurrentWaypointIndex`))
    (:`  `
      (bind _output_get (set `self.CurrentWaypointIndex` (`KismetMathLibrary.And_IntInt` _result (- (`KismetArrayLibrary.Array_Length` (`self.Waypoints`)) 1)))))))

(fn `GetNextWaypoint`
  (returns (NextWaypoint :type "/Game/BPs/AI/Waypoint Object Reference"))
  (bind _result (`/Engine/EditorBlueprintResources/StandardMacros.IncrementInt` (`self.CurrentWaypointIndex`))
    (:`  `
      (bind _output_get (set `self.CurrentWaypointIndex` (`KismetMathLibrary.And_IntInt` _result (- (`KismetArrayLibrary.Array_Length` (`self.Waypoints`)) 1))))
      (return (`|GetArrayItem` (`self.Waypoints`) _output_get)))))

(fn `Make Projectile Transform`
  (params (`Dist From Character` :type "Float (double-precision)") (`Projectile Scale` :type "Vector Structure"))
  (returns (ReturnValue :type "Transform Structure"))
  (bind _returnvalue (+ (`self.K2_GetActorLocation`) (* (`self.GetActorForwardVector`) `Dist From Character`)))
  (bind _asactor (cast `Actor` (`BlackboardComponent.GetValueAsObject` (`AIBlueprintHelperLibrary.GetBlackboard` null) (`self.TargetEnemy`))))
  (return (`KismetMathLibrary.MakeTransform` _returnvalue (`KismetMathLibrary.FindLookAtRotation` _returnvalue (`self.K2_GetActorLocation` _asactor)) `Projectile Scale`)))

(fn `UserConstructionScript`
  (`parent.UserConstructionScript`))