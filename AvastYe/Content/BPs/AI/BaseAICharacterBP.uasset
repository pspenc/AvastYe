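; Base AI character Blueprint that handles damage, death and reactions to other characters' deaths.
; While alive, taking damage launches it along the given vector and passes hitstun, damage and attacker to the BaseAIController to notify its behavior tree.
; Death runs the parent logic, plays a death animation on the mesh and destroys the actor after a delay.
; Kill reactions are forwarded to the same controller.
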(event `self.TakeDamage`
  (params (LaunchVector :type "Vector Structure") (`Incoming Damage` :type "Float (single-precision)") (Hitstun :type "Float (single-precision)") (Attacker :type "/Game/BPs/AI/BaseCharacterBP Object Reference"))
  (if (not (`self.Dead`))
    (`self.LaunchCharacter` LaunchVector true true)
    (bind _asbase_aicontroller (cast `/Game/BPs/AI/BaseAIController` (`self.GetController`)))
    (`/Game/BPs/AI/BaseAIController.NotifyBehaviorTreeOfDamage` _asbase_aicontroller Hitstun `Incoming Damage` Attacker)))

(event `self.Die`
  (`parent.Die`)
  (`SkeletalMeshComponent.PlayAnimation` (`self.Mesh`) "/Game/Assets/AnimStarterPack/Death_1.Death_1" false)
  (`KismetSystemLibrary.Delay` 20.0)
  (`self.K2_DestroyActor`))

(event `self.ReactToDeath`
  (params (KilledCharacter :type "/Game/BPs/AI/BaseCharacterBP Object Reference"))
  (bind _asbase_aicontroller (cast `/Game/BPs/AI/BaseAIController` (`self.GetController`)))
  (`/Game/BPs/AI/BaseAIController.ReactToDeath` _asbase_aicontroller KilledCharacter))

(fn `UserConstructionScript`
  (`parent.UserConstructionScript`))