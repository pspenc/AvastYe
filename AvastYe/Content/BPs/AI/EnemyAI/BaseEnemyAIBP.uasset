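; Base enemy character that fights with a child-actor melee weapon and shows health, targeting and quick-time indicators.
; It reports targets, attacks and death to a Director, and attack broadcasts set a blackboard flag when too many units share its target.
; Being hit by the Captain switches its target and briefly exempts it from that limit.
; Blockable melee swings use animations or timeline-driven weapon-pivot rotation; taunt and drop logic is disconnected.
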(event `InitHealthBar`
  (bind _enemyui (`self.EnemyUI`))
  (bind _asenemy_ui (cast `/Game/BPs/UI/Health/EnemyUI` (`WidgetComponent.GetUserWidgetObject` _enemyui)))
  (set `/Game/BPs/UI/Health/EnemyUI.Enemy` self _asenemy_ui)
  (`SceneComponent.SetVisibility` _enemyui true false)
  (set `/Game/BPs/UI/Health/EnemyUI.Size` (`self.HealthBarSize`) _asenemy_ui)
  (`/Game/BPs/UI/Health/EnemyUI.ChangeColor` _asenemy_ui (struct :`R` 1.0 :`B` 0.631373 :`A` 0.701961)))

(event `StartAttackBroadcast`
  ;[1 1 1] Broadcasting Attacks to allies
  (if (not (`self.InAttackBroadcast`))
    (set `self.InAttackBroadcast` true)
    (`/Game/BPs/AI/EnemyAIDIrector.UnitAttackingTarget` (`self.Director`) self (`self.CurrentTarget`))))

(event `self.ReceiveBeginPlay`
  (`parent.ReceiveBeginPlay`)
  (bind _asbase_melee_weapon_bp (cast `/Game/BPs/Weapons/BaseMeleeWeaponBP` (`ChildActorComponent.ChildActor` (`self.ChildActor`))))
  (set `self.Weapon` _asbase_melee_weapon_bp)
  (set `/Game/BPs/Weapons/BaseWeaponBP.WeaponOwner` self _asbase_melee_weapon_bp)
  (set `self.OriginalRot` (`SceneComponent.RelativeRotation` (`self.WeaponPivot`))))

(event `Get Targeted`
  (`SceneComponent.SetVisibility` (`self.TargetingIndicator`) true false)
  (`MeshComponent.SetScalarParameterValueOnMaterials` (`self.Mesh`) "FresnelInt" 50.0))

(event `EndAttackBroadcast`
  (bind _director (`self.Director`))
  ;[1 1 1] Broadcasting Attacks to allies
  (if (`self.InAttackBroadcast`)
    (`/Engine/EditorBlueprintResources/StandardMacros.IsValid` _director
      (:`Is Valid`
        (`/Game/BPs/AI/EnemyAIDIrector.UnitEndAttackingTarget` _director self (`self.CurrentTarget`))
        (`KismetSystemLibrary.Delay` 0.2)
        (set `self.InAttackBroadcast` false)))))

(event `Get UnTargeted`
  (`SceneComponent.SetVisibility` (`self.TargetingIndicator`) false false)
  (`MeshComponent.SetScalarParameterValueOnMaterials` (`self.Mesh`) "FresnelInt" 0.0))

(event `RecieveAttackBroadcast`
  (params (TargetEnemy :type "Actor Object Reference"))
  ;[1 1 1] Broadcasting Attacks to allies
  (if (== (`self.CurrentTarget`) TargetEnemy)
    (bind _result (`/Engine/EditorBlueprintResources/StandardMacros.IncrementInt` (`self.NumOtherAttackingMyTarget`))
      (:`  `
        (if (>= _result 2)
          (if (not (`self.IsCaptainTarget`))
            (`BlackboardComponent.SetValueAsBool` (`AIBlueprintHelperLibrary.GetBlackboard` null) (`self.TooManyAttackingTargetBBKey`) true)))))))

(event `/Game/BPs/Interfaces/DamagableInterface.getDamaged`
  (params (DamageDealt :type "Float (single-precision)") (DamageType :type "/Game/BPs/GlobalEnums/DamageTypes Enum" :default "NewEnumerator0") (EnemyTeamTag :type "GameplayTag Structure") (ForceVector :type "Vector Structure") (HitStun :type "Float (single-precision)") (Attacker :type "/Game/BPs/BaseCharacterBP Object Reference") (HitComponent :type "PrimitiveComponent Object Reference") (Sleep :type "Float (single-precision)"))
  (if (`BlueprintGameplayTagLibrary.HasTag` (`self.GameplayTags`) EnemyTeamTag true)
    (`self.AlertDirectorOfCOmbat`)
    (if (== (`GameplayStatics.GetObjectClass` Attacker) "/Game/BPs/CaptainCharacter.CaptainCharacter_C")
      (`self.BecomeCaptain'sTarget`)
      (`self.ChangeTarget` Attacker))
    (`parent.getDamaged` DamageDealt DamageType EnemyTeamTag ForceVector HitStun Attacker HitComponent Sleep)))

(event `BecomeCaptain'sTarget`
  (`BlueprintGameplayTagLibrary.AddGameplayTag` (`self.GameplayTags`) (struct :`TagName` "TargetingInfo.CaptainsTarget"))
  (set `self.IsCaptainTarget` true)
  (`KismetSystemLibrary.K2_SetTimerDelegate` (delegate `NoLongerCaptainsTarget`) 3.0)
  (`BlackboardComponent.SetValueAsBool` (`AIBlueprintHelperLibrary.GetBlackboard` null) (`self.TooManyAttackingTargetBBKey`) false))

(event `Taunt`
  ;[1 1 1] Taunt
)

(event `RecieveEndAttackBroadcast`
  (params (TargetEnemy :type "Actor Object Reference"))
  ;[1 1 1] Broadcasting Attacks to allies
  (if (== TargetEnemy (`self.CurrentTarget`))
    (bind _result (`/Engine/EditorBlueprintResources/StandardMacros.DecrementInt` (`self.NumOtherAttackingMyTarget`))
      (:`  `
        (if (< _result 2)
          (`BlackboardComponent.SetValueAsBool` (`AIBlueprintHelperLibrary.GetBlackboard` null) (`self.TooManyAttackingTargetBBKey`) false))))))

(event `TauntTick`
  ;[1 1 1] Taunt
)

(event `NoLongerCaptainsTarget`
  (`BlueprintGameplayTagLibrary.RemoveGameplayTag` (`self.GameplayTags`) (struct :`TagName` "TargetingInfo.CaptainsTarget"))
  (set `self.IsCaptainTarget` false))

(event `EndTaunt`
  ;[1 1 1] Taunt
)

(event `ChangeTarget`
  (params (Attacker :type "Actor Object Reference"))
  ;[1 1 1] Change Target
  (if (not (== Attacker (`self.CurrentTarget`)))
    (set `self.CurrentTarget` Attacker)
    (`/Game/BPs/AI/EnemyAIDIrector.UnitSwitchingTargets` (`self.Director`) self Attacker)))

(event `Sprint`
  (bind _charactermovement (`self.CharacterMovement`))
  (set `CharacterMovementComponent.MaxAcceleration` 100000.0 _charactermovement)
  (set `CharacterMovementComponent.MaxWalkSpeed` (`self.RunSpeed`) _charactermovement))

(event `UnSprint`
  (bind _charactermovement (`self.CharacterMovement`))
  (set `CharacterMovementComponent.MaxAcceleration` 1024.0 _charactermovement)
  (set `CharacterMovementComponent.MaxWalkSpeed` (`self.WalkSpeed`) _charactermovement))

(event `strafespeed`
  (set `CharacterMovementComponent.MaxWalkSpeed` 400.0 (`self.CharacterMovement`)))

(event `self.Die`
  (`self.AlertDirectorOfDeath`)
  (`self.EndAttackBroadcast`)
  (if (not (>= (`KismetMathLibrary.RandomIntegerInRange` 0 100) (`self.AmmoDropRate`)))
    (`self.Drop Ammo`))
  (`parent.Die`))

(event `Drop Ammo`
  ;[1 0.2493 0] Disconnected
)

(event `AlertDirectorOfDeath`
  (bind _director (`self.Director`))
  (`/Engine/EditorBlueprintResources/StandardMacros.IsValid` _director
    (:`Is Valid`
      (`/Game/BPs/AI/EnemyAIDIrector.UnitHasDied` _director self))))

(event `AlertDirectorOfCombat`)

(event `self.MeleeAttack`
  (bind _weapon (`self.Weapon`))
  (bind _returnvalue (`BlackboardComponent.GetValueAsObject` (`AIBlueprintHelperLibrary.GetBlackboard` null) (`self.TargetEnemy`)))
  (bind _asbase_character_bp (cast `/Game/BPs/BaseCharacterBP` _returnvalue))
  (message `/Game/BPs/Interfaces/GameModeInterface.CharacterAttacking` (`GameplayStatics.GetGameMode`) self _asbase_character_bp)
  (bind _ascaptain_character (cast `/Game/BPs/CaptainCharacter` _returnvalue)
    (:`then`
      (`/Game/BPs/CaptainCharacter.NotifyPlayerOfMelee` _ascaptain_character self)
      (if (`self.usesAnimations`)
        (`SkeletalMeshComponent.PlayAnimation` (`self.Mesh`) "/Game/Assets/Cockroach/ChargingHeavy.ChargingHeavy" false)
        (`KismetSystemLibrary.Delay` 0.2)
        (set `self.IsAttacking` true)
        (`/Game/BPs/Weapons/BaseMeleeWeaponBP.InitialTraceAttack` _weapon)
        (`SkeletalMeshComponent.PlayAnimation` (`self.Mesh`) "/Game/Assets/Cockroach/cockroach_heavyAttack_combo_1.cockroach_heavyAttack_combo_1" false)
        (`KismetSystemLibrary.Delay` 0.8)
        (set `self.IsAttacking` false)
        (`SkeletalMeshComponent.SetAnimationMode` (`self.Mesh`) "AnimationBlueprint")
        (`/Game/BPs/Weapons/BaseMeleeWeaponBP.Clear Hit Actors Array` _weapon)
        (else
          (bind (_direction _newtrack_0) (`Timeline|WindupTimeline` :!via `PlayFromStart` :!label _label)
            (:`Update`
              (`SceneComponent.K2_SetRelativeRotation` (`self.WeaponPivot`) (`KismetMathLibrary.RLerp` (struct :`Pitch` -40.0) (struct :`Pitch` -70.0 :`Yaw` 80.0) _newtrack_0) false false))
            (:`Finished`
              (set `self.IsAttacking` true)
              (`/Game/BPs/Weapons/BaseMeleeWeaponBP.InitialTraceAttack` (`self.Weapon`))
              (bind (_direction_2 _newtrack_0_2) (`Timeline|SwingTimeline` :!via `PlayFromStart` :!label _label_2)
                (:`Update`
                  (`/Engine/EditorBlueprintResources/StandardMacros.IsValid` (`self.SwingTimeline`)
                    (:`Is Valid`
                      (`SceneComponent.K2_SetRelativeRotation` (`self.WeaponPivot`) (`KismetMathLibrary.RLerp` (struct :`Pitch` -70.0 :`Yaw` 80.0) (struct :`Pitch` -90.0 :`Yaw` -75.0) _newtrack_0_2) false false))))
                (:`Finished`
                  (set `self.IsAttacking` false)
                  (`KismetSystemLibrary.Delay` 0.1)
                  (bind (_direction_3 _newtrack_0_3) (`Timeline|ReturnTimeline` :!via `PlayFromStart`)
                    (:`Update`
                      (`SceneComponent.K2_SetRelativeRotation` (`self.WeaponPivot`) (`KismetMathLibrary.RLerp` (struct :`Pitch` -90.0 :`Yaw` -75.0) (struct :`Pitch` -40.0) _newtrack_0_3) false false)
                      (`/Game/BPs/Weapons/BaseMeleeWeaponBP.Clear Hit Actors Array` (`self.Weapon`)))))))))))
    (:`CastFailed`
      (goto _label :!via `PlayFromStart`))))

(event `AttackGotBlocked`
  (bind _weapon (`self.Weapon`))
  (bind _weaponpivot (`self.WeaponPivot`))
  (if (`self.usesAnimations`)
    (set `self.IsAttacking` false)
    (`SkeletalMeshComponent.PlayAnimation` (`self.Mesh`) "/Game/Assets/Cockroach/cockroach_block01.cockroach_block01" false)
    (`KismetSystemLibrary.Delay` 0.2)
    (`SkeletalMeshComponent.SetAnimationMode` (`self.Mesh`) "AnimationBlueprint")
    (`/Game/BPs/Weapons/BaseMeleeWeaponBP.Clear Hit Actors Array` (`self.Weapon`))
    (else
      (`|ExecutionSequence`
        (:`then_0`
          (`/Engine/EditorBlueprintResources/StandardMacros.IsValid` (`self.SwingTimeline`)
            (:`Is Valid`
              (goto _label_2 :!via `Stop`))))
        (:`then_1`
          (`/Engine/EditorBlueprintResources/StandardMacros.IsValid` _weaponpivot
            (:`Is Valid`
              (`SceneComponent.K2_SetRelativeRotation` _weaponpivot (`self.OriginalRot`) false false))))
        (:`then_2`
          (set `self.IsAttacking` false))
        (:`then_3`
          (`/Engine/EditorBlueprintResources/StandardMacros.IsValid` _weapon
            (:`Is Valid`
              (`/Game/BPs/Weapons/BaseMeleeWeaponBP.Clear Hit Actors Array` _weapon))))))))

(event `WaitForDirector`
  (cast `Actor` (`BlackboardComponent.GetValueAsObject` (`AIBlueprintHelperLibrary.GetBlackboard` null) (`self.TargetEnemy`)))
  (`/Game/BPs/AI/EnemyAIDIrector.UnitWaitingforDirection` (`self.Director`) self))

(event `TurnOnInteractWidget`
  (params (Icon :type "/Game/BPs/GlobalEnums/QuickTimeEnum Enum" :default "NewEnumerator0"))
  (bind _asenemy_ui (cast `/Game/BPs/UI/Health/EnemyUI` (`WidgetComponent.GetUserWidgetObject` (`self.EnemyUI`))))
  (`/Game/BPs/UI/Health/EnemyUI.SetIcon` _asenemy_ui Icon)
  (`/Game/BPs/UI/Health/EnemyUI.On` _asenemy_ui))

(event `/Game/BPs/Interfaces/DamagableInterface.becomeQuickTimeTarget`
  (params (QuickTimeType :type "/Game/BPs/GlobalEnums/QuickTimeEnum Enum" :default "NewEnumerator0"))
  (`parent.becomeQuickTimeTarget` QuickTimeType)
  (`self.TurnOnInteractWidget` QuickTimeType))

(event `TurnOffInteractWidget`
  (bind _asenemy_ui (cast `/Game/BPs/UI/Health/EnemyUI` (`WidgetComponent.GetUserWidgetObject` (`self.EnemyUI`))))
  (`/Game/BPs/UI/Health/EnemyUI.Off` _asenemy_ui))

(event `/Game/BPs/Interfaces/DamagableInterface.clearSelfAsQuickTimeTarget`
  (`parent.clearSelfAsQuickTimeTarget`)
  (`self.TurnOffInteractWidget`))

(event `/Game/BPs/Interfaces/DamagableInterface.clearQuickTimeTarget`
  (`parent.clearQuickTimeTarget`)
  (`self.TurnOffInteractWidget`))

(fn `ReportTargetsToDirector`
  (params (NewParam :type "Array of Actor Object Reference"))
  (returns (DecidedTarget :type "Actor Object Reference"))
  (bind _decidedtarget (`/Game/BPs/AI/EnemyAIDIrector.DecideTargetForUnit` (`self.Director`) self NewParam))
  (return _decidedtarget))

(fn `UserConstructionScript`
  (`parent.UserConstructionScript`))