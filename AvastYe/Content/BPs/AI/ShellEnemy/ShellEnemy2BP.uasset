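; Shell enemy variant that ignores damage until one specific damage type flips it over, exposing it for a limited time.
; The damage override passes hits to the parent only while flipped; otherwise the matching type triggers the flip without dealing damage.
; Flipping rotates and offsets the mesh, swaps its material, recolors the health bar and sets a Blackboard flag for the AI, then reverts after a delay.
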(event `self.InitHealthBar`
  (`parent.InitHealthBar`)
  (bind _asenemy_health (cast `/Game/BPs/UI/Health/EnemyHealth` (`WidgetComponent.GetUserWidgetObject` (`self.WidgetHealth`))))
  (`/Game/BPs/UI/Health/EnemyHealth.ChangeColor` _asenemy_health (struct :`R` 1.0 :`G` 0.341915 :`A` 0.701961)))

(event `self.ReceiveBeginPlay`
  (`parent.ReceiveBeginPlay`))

(event `self.getDamaged`
  (params (DamageDealt :type "Float (single-precision)") (DamageType :type "/Game/BPs/GlobalEnums/DamageTypes Enum" :default "NewEnumerator0") (EnemyTeamTag :type "GameplayTag Structure") (ForceVector :type "Vector Structure") (HitStun :type "Float (single-precision)") (Attacker :type "/Game/BPs/BaseCharacterBP Object Reference") (HitComponent :type "PrimitiveComponent Object Reference"))
  (if (`self.Flipped`)
    (`parent.getDamaged` DamageDealt DamageType EnemyTeamTag ForceVector HitStun Attacker HitComponent)
    (elif (`|EnumEquality` DamageType "NewEnumerator3")
      (`self.Get Flipped`))))

(event `Get Flipped`
  (bind _mesh (`self.Mesh`))
  (bind _asenemy_health (cast `/Game/BPs/UI/Health/EnemyHealth` (`WidgetComponent.GetUserWidgetObject` (`self.WidgetHealth`))))
  (`/Game/BPs/UI/Health/EnemyHealth.ChangeColor` _asenemy_health (struct :`R` 1.0 :`B` 0.630757 :`A` 1.0))
  (`SceneComponent.K2_AddLocalRotation` _mesh (struct :`Roll` 180.0) false false)
  (`SceneComponent.K2_AddLocalOffset` _mesh (0.0 0.0 -100.0) false false)
  (`PrimitiveComponent.SetMaterial` _mesh 0 "/Game/Assets/Temp/GlowingYellow.GlowingYellow")
  (bind _output_get (set `self.Flipped` true))
  (`BlackboardComponent.SetValueAsBool` (`AIBlueprintHelperLibrary.GetBlackboard` null) (`self.FlippedBBKey`) _output_get)
  (`KismetSystemLibrary.Delay` (`self.FlipDuration`))
  (`SceneComponent.K2_AddLocalRotation` _mesh (struct :`Roll` 180.0) false false)
  (`SceneComponent.K2_AddLocalOffset` _mesh (0.0 0.0 -100.0) false false)
  (`PrimitiveComponent.SetMaterial` _mesh 0 "/Game/Assets/Temp/Red2.Red2")
  (bind _output_get_2 (set `self.Flipped` false))
  (`BlackboardComponent.SetValueAsBool` (`AIBlueprintHelperLibrary.GetBlackboard` null) (`self.FlippedBBKey`) _output_get_2)
  (`/Game/BPs/UI/Health/EnemyHealth.ChangeColor` _asenemy_health (struct :`R` 1.0 :`G` 0.341915 :`A` 0.701961)))

(fn `UserConstructionScript`
  (`parent.UserConstructionScript`))