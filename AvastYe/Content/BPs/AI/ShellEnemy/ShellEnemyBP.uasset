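; Shell enemy Blueprint that can only be damaged while flipped over.
; When upright, it ignores incoming hits except one damage type, which triggers the flip without passing damage on.
; Flipping rotates the actor 180 degrees and sets a Flipped flag, then a five-second delay rights it again.
; While flipped, hits are forwarded to the parent class's damage handling.
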(event `/Game/BPs/Interfaces/DamagableInterface.getDamaged`
  (params (DamageDealt :type "Float (single-precision)") (DamageType :type "/Game/BPs/GlobalEnums/DamageTypes Enum" :default "NewEnumerator0") (EnemyTeamTag :type "GameplayTag Structure") (ForceVector :type "Vector Structure") (HitStun :type "Float (single-precision)") (Attacker :type "/Game/BPs/BaseCharacterBP Object Reference") (HitComponent :type "PrimitiveComponent Object Reference"))
  (if (`self.Flipped`)
    (`parent.getDamaged` DamageDealt DamageType EnemyTeamTag ForceVector HitStun Attacker HitComponent)
    (elif (`|EnumEquality` DamageType "NewEnumerator3")
      (`self.Get Flipped`))))

(event `Get Flipped`
  (`self.K2_AddActorLocalRotation` (struct :`Roll` 180.0))
  (set `self.Flipped` true)
  (`KismetSystemLibrary.Delay` 5.0)
  (`self.K2_AddActorLocalRotation` (struct :`Roll` 180.0))
  (set `self.Flipped` false))

(fn `UserConstructionScript`
  (`parent.UserConstructionScript`))