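; Base character Blueprint providing walk/run speeds, health, and team-based combat through gameplay tags.
; Data-driven attacks feed windup projectile shots and forward-impulse melee hitbox combos with input queuing and a timed reset.
; Damage filters by team tag, launches the character, then either kills it by tagging Dead or applies timer-based hitstun, notifying the controller.
; Scary-attack and death reactions are empty events, with the former bound to an AvastYeGameMode broadcast.
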(event `Walk`
  ;[1 1 1] Movement Logic
  (set `CharacterMovementComponent.MaxWalkSpeed` (`self.WalkSpeed`) (`self.CharacterMovement`)))

(event `Key|LeftShift`
  (params (Key :type "Key Structure"))
  ;[1 1 1] Movement Logic
)

(event `Run`
  ;[1 1 1] Movement Logic
  (set `CharacterMovementComponent.MaxWalkSpeed` (`self.RunSpeed`) (`self.CharacterMovement`)))

(event `self.ReceiveBeginPlay`
  ;[1 1 1] Begin Play
  (bind _asavast_ye_game_mode (cast `/Game/BPs/AvastYeGameMode` (`GameplayStatics.GetGameMode`)))
  (add `/Game/BPs/AvastYeGameMode.BroadcastScaryAttack` _asavast_ye_game_mode (delegate `ReactToScaryAttack`))
  (set `self.MaxHealth` (`self.Health`))
  (set `CharacterMovementComponent.MaxWalkSpeed` (`self.WalkSpeed`) (`self.CharacterMovement`))
  (if (`GameplayTagAssetInterface.HasMatchingGameplayTag` self (struct :`TagName` "Team.BadGuy"))
    (set `self.EnemyTeamTag` (struct :`TagName` "Team.GoodGuy")) ; If i am bad guy. Then enemy is good guy
    (else
      (set `self.EnemyTeamTag` (struct :`TagName` "Team.BadGuy")) ; If I not bad guy. Im good guy. And my enemy is bad guy
    )))

(event `ReactToScaryAttack`
  ;[1 1 1] Begin Play
)

(event `RangedAttack`
  (bind (_initdistfromshooter _windup _winddown _projectilescale _projectiletofire) (break `/Game/BPs/Structs/RangedAttackStruct` (`|GetArrayItem` (`self.RangedAttackList`))))
  ;[1 1 1] Ranged Attack Logic
  (set `self.InputEnabled` false)
  (`KismetSystemLibrary.Delay` _windup)
  (bind _returnvalue (`self.Make Projectile Transform` _initdistfromshooter _projectilescale))
  (`|SpawnActorFromClass` _projectiletofire _returnvalue "Undefined" "OverrideRootScale" self (`self.EnemyTeamTag`) self null)
  (set `self.InputEnabled` true))

(event `MeleeAttack`
  (bind _attacks (`self.Attacks`))
  (bind _attackcount (`self.AttackCount`))
  (bind _output (`|GetArrayItem` _attacks _attackcount))
  ;[1 1 1] Melee Attack Logic
  (if (`self.IsAttacking`)
    (set `self.AttackQueued` true)
    (else
      (set `self.InputEnabled` false)
      (set `self.IsAttacking` true)
      (`self.AddForwardMovement` (`.MoveForwardAmount_31_A178A4244E5BC38A9EADE3AAF553B29D` (break `/Game/BPs/Structs/HitboxAttackStruct` _output)))
      (`/Game/BPs/MacroFunctionLibraries/AvastYeActorMacros.HitboxAttack` _output (`self.EnemyTeamTag`) self
        (:`Done`
          (if (< _attackcount (- (`KismetArrayLibrary.Array_Length` _attacks) 1))
            (`/Engine/EditorBlueprintResources/StandardMacros.IncrementInt` _attackcount
              (:`  `
                (`KismetSystemLibrary.K2_SetTimerDelegate` (delegate `ResetAtkCount`) 1.0)
                (set `self.InputEnabled` true)
                (`KismetSystemLibrary.Delay` 0.35)))
            (else
              (`self.ResetAtkCount`)
              (set `self.InputEnabled` true)
              (`KismetSystemLibrary.Delay` 0.75)))
          (set `self.IsAttacking` false)
          (if (`self.AttackQueued`)
            (set `self.AttackQueued` false)
            (`self.MeleeAttack`)))))))

(event `ResetAtkCount`
  ;[1 1 1] Melee Attack Logic
  (set `self.AttackCount` 0)
  (set `self.AttackQueued` false))

(event `/Game/BPs/Interfaces/DamagableInterface.getDamaged`
  (params (DamageDealt :type "Float (single-precision)") (DamageType :type "/Game/BPs/GlobalEnums/DamageTypes Enum" :default "NewEnumerator0") (EnemyTeamTag :type "GameplayTag Structure") (ForceVector :type "Vector Structure") (HitStun :type "Float (single-precision)") (Attacker :type "/Game/BPs/BaseCharacterBP Object Reference") (HitComponent :type "PrimitiveComponent Object Reference"))
  (if (`self.Dead`)
    _
    (elif (`BlueprintGameplayTagLibrary.HasTag` (`self.GameplayTags`) EnemyTeamTag true)
      (`self.LaunchCharacter` ForceVector true true)
      (bind _output_get (set `self.Health` (- (`self.Health`) DamageDealt)))
      (if (<= _output_get 0.0)
        (set `self.Dead` true)
        (`self.Die`)
        (elif (> HitStun 0.0)
          (`self.Hitstun` HitStun)
          (else
            (message `/Game/BPs/Interfaces/AICommunicationInterface.ControllerReactToDamage` (`self.GetController`) 0.0 (`self.Health`) Attacker)))))))

(event `MoveWithAttack`
  (`CharacterMovementComponent.AddImpulse` (`self.CharacterMovement`) (* (`self.GetActorForwardVector`) 250000.0) false))

(event `EndHitStun`
  (set `self.InputEnabled` true))

(event `Hitstun`
  (params (StunLength :type "Float (double-precision)"))
  (if (> StunLength (`KismetSystemLibrary.K2_GetTimerRemainingTimeHandle` (stale _returnvalue)))
    (set `self.InputEnabled` false)
    (bind _returnvalue (`KismetSystemLibrary.K2_SetTimerDelegate` (delegate `EndHitStun`) StunLength))
    (message `/Game/BPs/Interfaces/AICommunicationInterface.ControllerReactToDamage` (`self.GetController`) StunLength (`self.Health`) null)))

(event `ReactToDeath`
  (params (KilledCharacter :type "/Game/BPs/BaseCharacterBP Object Reference")))

(event `Die`
  (`BlueprintGameplayTagLibrary.AddGameplayTag` (`self.GameplayTags`) (struct :`TagName` "Dead"))
  (set `self.Dead` true))

(event `AttackMovement`
  (params (Distance :type "Float (double-precision)"))
  (bind _charactermovement (`self.CharacterMovement`))
  ;[1 1 1] Attack Movement
  (set `CharacterMovementComponent.GroundFriction` 1.0 _charactermovement)
  (`CharacterMovementComponent.AddImpulse` _charactermovement (* (`self.GetActorForwardVector`) Distance) true)
  (`KismetSystemLibrary.Delay` 0.25)
  (set `CharacterMovementComponent.GroundFriction` 8.0 _charactermovement))

(event `Get Healed`
  (params (`Amount Healed` :type "Float (double-precision)"))
  (bind _returnvalue (+ `Amount Healed` (`self.Health`)))
  (if (> _returnvalue (`self.MaxHealth`))
    (set `self.Health` (`self.MaxHealth`))
    (else
      (set `self.Health` _returnvalue))))

(fn `AddForwardMovement`
  (params (ForwardImpulse :type "Float (double-precision)"))
  (`CharacterMovementComponent.AddImpulse` (`self.CharacterMovement`) (* (`self.GetActorForwardVector`) ForwardImpulse) false))

(fn `Make Projectile Transform`
  (params (`Dist From Character` :type "Float (double-precision)") (`Projectile Scale` :type "Vector Structure"))
  (returns (ReturnValue :type "Transform Structure"))
  (return (`KismetMathLibrary.MakeTransform` (+ (`self.K2_GetActorLocation`) (* (`self.GetActorForwardVector`) `Dist From Character`)) (`self.K2_GetActorRotation`) `Projectile Scale`)))

(fn `UserConstructionScript`)