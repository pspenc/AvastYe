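; Base enemy character that assigns its team and enemy object type in the construction script and hands combat events to its BasicEnemyController.
; While alive, taking damage launches it with a full velocity override and has the controller notify the behavior tree of damage and hitstun.
; Another character's death is forwarded to the controller, with a leftover debug print.
; Its own death runs parent logic, plays a death animation, then destroys the actor after a delay.
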(event `self.TakeDamage`
  (params (LaunchVector :type "Vector Structure") (`Incoming Damage` :type "Float (single-precision)") (Hitstun :type "Float (single-precision)"))
  (if (not (`self.Dead`))
    (`self.LaunchCharacter` LaunchVector true true)
    (bind _asbasic_enemy_controller (cast `/Game/BPs/AI/EnemyAI/BasicEnemyController` (`self.GetController`)))
    (`/Game/BPs/AI/EnemyAI/BasicEnemyController.NotifyBehaviorTreeOfDamage` _asbasic_enemy_controller Hitstun `Incoming Damage`)))

(event `self.Die`
  (`parent.Die`)
  (`SkeletalMeshComponent.PlayAnimation` (`self.Mesh`) "/Game/Assets/AnimStarterPack/Death_1.Death_1" false)
  (`KismetSystemLibrary.Delay` 20.0)
  (`self.K2_DestroyActor`))

(event `self.ReactToDeath`
  (params (`Killed Character` :type "/Game/BPs/BaseCharacterBP Object Reference"))
  (`KismetSystemLibrary.PrintString` "Hello")
  (bind _asbasic_enemy_controller (cast `/Game/BPs/AI/EnemyAI/BasicEnemyController` (`self.GetController`)))
  (`/Game/BPs/AI/EnemyAI/BasicEnemyController.NotifyOfDeath` _asbasic_enemy_controller `Killed Character`))

(fn `UserConstructionScript`
  (`parent.UserConstructionScript`)
  (set `self.Team` "NewEnumerator1")
  (set `self.EnemyTeam` "ObjectTypeQuery7"))