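; Player Captain character who fights and commands a crew of three ants.
; Holding right mouse enters captaining mode: an over-shoulder aim with reticle, gated hover traces on interactables, and left click firing a pistol instead of meleeing.
; Number keys select an ant, and in that mode a camera trace writes its Blackboard state plus target object or location.
; Taking damage sends the crew's AI controllers into combat, and hits can destroy captain-required interactables.
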(event `self.ReceiveBeginPlay`
  (bind _the_crew (`self.The Crew`))
  (bind _bullant (`self.BullAnt`))
  ;[1 1 1] Begin Play
  (`KismetArrayLibrary.Array_Add` _the_crew _bullant)
  (`KismetArrayLibrary.Array_Add` _the_crew (`self.CarpenterAnt`))
  (`KismetArrayLibrary.Array_Add` _the_crew (`self.FireAnt`))
  (set `self.CurrentlySelectedAnt` _bullant))

(event `self.ReceiveTick`
  (params (DeltaSeconds :type "Float (single-precision)"))
  (bind _follow_camera (`self.Follow Camera`))
  (bind _returnvalue (`SceneComponent.K2_GetComponentLocation` _follow_camera))
  ;[1 1 1] Event Tick/Captaining hover effect
  (`/Engine/EditorBlueprintResources/StandardMacros.Gate` true :!label _label
    (:`Exit`
      (bind _outhit (`KismetSystemLibrary.LineTraceSingle` _returnvalue (+ _returnvalue (* (`SceneComponent.GetForwardVector` _follow_camera) 5000.0)) "TraceTypeQuery2" false (`self.The Crew`) "None" true (struct :`R` 1.0 :`A` 1.0) (struct :`G` 1.0 :`A` 1.0) 0.1))
      (bind (_bblockinghit _binitialoverlap _time _distance _location _impactpoint _normal _impactnormal _physmat _hitactor) (`GameplayStatics.BreakHitResult` _outhit))
      (if (`KismetMathLibrary.ClassIsChildOf` (`GameplayStatics.GetObjectClass` _hitactor) "/Game/BPs/PuzzleInteractables/InteractableObject.InteractableObject_C")
        (bind _asinteractable_object (cast `/Game/BPs/PuzzleInteractables/InteractableObject` _hitactor))
        (`/Game/BPs/PuzzleInteractables/InteractableObject.OnHovered` _asinteractable_object)))))

(event `Start Captaining`
  ;[1 1 1] Event Tick/Captaining hover effect
  (goto _label :!via `Open`))

(event `Stop Captaining`
  ;[1 1 1] Event Tick/Captaining hover effect
  (goto _label :!via `Close`))

(event `self.ReceiveActorBeginOverlap`
  (params (OtherActor :type "Actor Object Reference"))
  ;[1 1 1] Check Interactable on Overlap
  (if (== (`GameplayStatics.GetObjectClass` OtherActor) "/Game/BPs/PuzzleInteractables/InteractableObject.InteractableObject_C")
    (set `self.isNearInterObject` true)
    (bind _asinteractable_object (cast `/Game/BPs/PuzzleInteractables/InteractableObject` OtherActor))
    (set `self.CloseInterObject` _asinteractable_object)))

(event `Crew Command`
  (bind _follow_camera (`self.Follow Camera`))
  (bind _returnvalue (`AIBlueprintHelperLibrary.GetBlackboard` (`self.CurrentlySelectedAnt`)))
  (bind _returnvalue_2 (`AIBlueprintHelperLibrary.GetBlackboard` (`self.CurrentlySelectedAnt`)))
  (bind _returnvalue_3 (`SceneComponent.K2_GetComponentLocation` _follow_camera))
  ;[1 1 1] Captain Command
  (if (`self.Captaining Mode On`)
    (bind _outhit (`KismetSystemLibrary.LineTraceSingle` _returnvalue_3 (+ _returnvalue_3 (* (`SceneComponent.GetForwardVector` _follow_camera) 5000.0)) "TraceTypeQuery2" false (`self.The Crew`) "ForDuration" true (struct :`R` 1.0 :`A` 1.0) (struct :`G` 1.0 :`A` 1.0) 2.0))
    (bind (_bblockinghit _binitialoverlap _time _distance _location _impactpoint _normal _impactnormal _physmat _hitactor) (`GameplayStatics.BreakHitResult` _outhit))
    (if (`KismetMathLibrary.ClassIsChildOf` (`GameplayStatics.GetObjectClass` _hitactor) "/Game/BPs/PuzzleInteractables/InteractableObject.InteractableObject_C")
      (`BlackboardComponent.SetValueAsEnum` _returnvalue_2 (`self.PuzzleAIState`) (enumliteral `/Game/BPs/AI/AI_PuzzleStates` "NewEnumerator2"))
      (bind _asinteractable_object (cast `/Game/BPs/PuzzleInteractables/InteractableObject` _hitactor))
      (`BlackboardComponent.SetValueAsObject` _returnvalue_2 (`self.InterObject`) _asinteractable_object)
      (else
        (`BlackboardComponent.SetValueAsVector` _returnvalue (`self.TargetLocation`) _location)
        (`BlackboardComponent.SetValueAsEnum` _returnvalue (`self.PuzzleAIState`) (enumliteral `/Game/BPs/AI/AI_PuzzleStates` "NewEnumerator1"))))))

(event `self.ReceiveActorEndOverlap`
  (params (OtherActor :type "Actor Object Reference"))
  ;[1 1 1] Check Interactable on Overlap
  (set `self.isNearInterObject` false)
  (set `self.CloseInterObject` null))

(event `Key|One`
  (params (Key :type "Key Structure"))
  ;[1 1 1] Crew Command
  (:`Pressed`
    (set `self.CurrentlySelectedAnt` (`self.BullAnt`))
    (`self.Crew Command` :!label _label_2)))

(event `Key|Two`
  (params (Key :type "Key Structure"))
  ;[1 1 1] Crew Command
  (:`Pressed`
    (set `self.CurrentlySelectedAnt` (`self.CarpenterAnt`))
    (goto _label_2)))

(event `Key|Three`
  (params (Key :type "Key Structure"))
  ;[1 1 1] Crew Command
  (:`Pressed`
    (set `self.CurrentlySelectedAnt` (`self.FireAnt`))
    (goto _label_2)))

(event `Key|RightMouseButton`
  (params (Key :type "Key Structure"))
  (bind _charactermovement (`self.CharacterMovement`))
  (bind _springarm (`self.SpringArm`))
  (bind _follow_camera (`self.Follow Camera`))
  ;[1 1 1] "Captaining" Mode
  (:`Pressed`
    (set `self.Captaining Mode On` true)
    (set `SpringArmComponent.TargetArmLength` 250.0 _springarm)
    (set `SpringArmComponent.SocketOffset` (0.0 100.0 -20.0) _springarm)
    (`CameraComponent.SetFieldOfView` _follow_camera 90.0)
    (bind _output_get (set `CameraComponent.bUsePawnControlRotation` true _follow_camera))
    (set `self.bUseControllerRotationYaw` _output_get)
    (set `CharacterMovementComponent.bOrientRotationToMovement` false _charactermovement)
    (bind _returnvalue (`|CreateWidget` "/Game/BPs/reticle.reticle_C" (`GameplayStatics.GetPlayerController` 0)))
    (`UserWidget.AddToViewport` _returnvalue 0)
    (`self.Start Captaining`))
  (:`Released`
    (set `self.Captaining Mode On` false)
    (set `SpringArmComponent.TargetArmLength` 300.0 _springarm)
    (set `SpringArmComponent.SocketOffset` (0.0 0.0 0.0) _springarm)
    (`CameraComponent.SetFieldOfView` _follow_camera 90.0)
    (bind _output_get_2 (set `CameraComponent.bUsePawnControlRotation` false _follow_camera))
    (set `self.bUseControllerRotationYaw` _output_get_2)
    (set `CharacterMovementComponent.bOrientRotationToMovement` true _charactermovement)
    (`WidgetLayoutLibrary.RemoveAllWidgets`)
    (`self.Stop Captaining`)))

(event `self.TakeDamage`
  (params (LaunchVector :type "Vector Structure") (`Incoming Damage` :type "Float (single-precision)") (Hitstun :type "Float (single-precision)") (Attacker :type "/Game/BPs/AI/BaseCharacterBP Object Reference"))
  ;[1 1 1] Take Damage
  (`parent.TakeDamage` LaunchVector `Incoming Damage` Hitstun Attacker)
  (for _array_element (`self.The Crew`)
    (bind _ascrew_aicontroller (cast `/Game/BPs/AI/CrewAIController` (`self.GetController` _array_element)))
    (`/Game/BPs/AI/CrewAIController.EnterCombat` _ascrew_aicontroller Attacker)))

(event `Key|LeftMouseButton`
  (params (Key :type "Key Structure"))
  ;[1 1 1] Left Mouse Control
  (:`Pressed`
    (if (`self.Captaining Mode On`)
      (`self.Shoot Pistol`)
      (else
        (`self.MeleeAttack`)))))

(event `Shoot Pistol`
  (bind _follow_camera (`self.Follow Camera`))
  (bind _returnvalue (`SceneComponent.K2_GetComponentLocation` _follow_camera))
  (bind _returnvalue_2 (`SceneComponent.GetSocketLocation` (`self.Mesh`) "hand_r"))
  (bind _returnvalue_3 (+ _returnvalue_2 (`self.GetActorForwardVector`)))
  ;[1 1 1] Shoot
  (if (`self.Can Shoot`)
    (set `self.InputEnabled` false)
    (set `self.Can Shoot` false)
    (`KismetSystemLibrary.Delay` 0.2)
    (bind (_outhit _returnvalue_4) (`KismetSystemLibrary.LineTraceSingle` :`Start` _returnvalue :`End` (+ _returnvalue (* (`SceneComponent.GetForwardVector` _follow_camera) 5000.0)) :`TraceChannel` "TraceTypeQuery2" :`DrawTime` 2.0))
    (if _returnvalue_4
      (`|SpawnActorFromClass` "/Game/BPs/CaptainBullet.CaptainBullet_C" (`KismetMathLibrary.MakeTransform` _returnvalue_3 (`KismetMathLibrary.FindLookAtRotation` _returnvalue_2 (`.ImpactPoint` (`GameplayStatics.BreakHitResult` _outhit)))) "AdjustIfPossibleButAlwaysSpawn" "OverrideRootScale" null self)
      (else
        (`|SpawnActorFromClass` "/Game/BPs/CaptainBullet.CaptainBullet_C" (`KismetMathLibrary.MakeTransform` _returnvalue_3 (`SceneComponent.K2_GetComponentRotation` (`self.Follow Camera`))) "AdjustIfPossibleButAlwaysSpawn" "OverrideRootScale" null self)
        (`KismetSystemLibrary.Delay` 0.2)))
    (set `self.InputEnabled` true)
    (`KismetSystemLibrary.Delay` 0.5)
    (set `self.Can Shoot` true)))

(event `Key|E`
  (params (Key :type "Key Structure"))
  (:`Pressed`
    (if (`self.Captaining Mode On`)
      _)))

(event `self.OnHitNonCharacter`
  (params (HitActor :type "Actor Object Reference"))
  (bind _asinteractable_object (cast `/Game/BPs/PuzzleInteractables/InteractableObject` HitActor))
  (if (`/Game/BPs/PuzzleInteractables/InteractableObject.CaptainRequired` _asinteractable_object)
    (`self.K2_DestroyActor` _asinteractable_object)))

(fn `Make Projectile Transform`
  (params (`Dist From Character` :type "Float (double-precision)") (`Projectile Scale` :type "Vector Structure"))
  (returns (ReturnValue :type "Transform Structure"))
  (bind _follow_camera (`self.Follow Camera`))
  (bind _returnvalue (`SceneComponent.K2_GetComponentLocation` _follow_camera))
  (bind _returnvalue_2 (`SceneComponent.GetSocketLocation` (`self.Mesh`) "hand_r"))
  (bind _returnvalue_3 (+ _returnvalue_2 (`self.GetActorForwardVector`)))
  (bind (_outhit _returnvalue_4) (`KismetSystemLibrary.LineTraceSingle` :`Start` _returnvalue :`End` (+ _returnvalue (* (`SceneComponent.GetForwardVector` _follow_camera) 5000.0)) :`TraceChannel` "TraceTypeQuery2" :`DrawTime` 2.0))
  (if _returnvalue_4
    (return (`KismetMathLibrary.MakeTransform` _returnvalue_3 (`KismetMathLibrary.FindLookAtRotation` _returnvalue_2 (`.ImpactPoint` (`GameplayStatics.BreakHitResult` _outhit))) `Projectile Scale`))
    (else
      (return (`KismetMathLibrary.MakeTransform` _returnvalue_3 (`SceneComponent.K2_GetComponentRotation` (`self.Follow Camera`)) `Projectile Scale`)))))

(fn `UserConstructionScript`
  (`parent.UserConstructionScript`))