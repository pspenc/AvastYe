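; Base melee weapon Blueprint that deals damage when its collision overlaps another actor during its owner's attack.
; It picks heavy or light damage, knockback and knock-up from the owner's attack state, with shorter hit stun for light hits.
; The hit is sent through GetDamagedMessage with directional force and the owner's enemy team tag.
; A hit particle spawns at the weapon's location, scaled up for heavy attacks.
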(event `self.WeaponCollision.OnComponentBeginOverlap`
  (params (OverlappedComponent :type "PrimitiveComponent Object Reference") (OtherActor :type "Actor Object Reference") (OtherComp :type "PrimitiveComponent Object Reference") (OtherBodyIndex :type Integer) (bFromSweep :type Boolean) (SweepResult :type "HitResult Structure (by ref)"))
  (bind _returnvalue (`self.K2_GetActorLocation`))
  (bind _weaponowner (`self.WeaponOwner`))
  (bind _enemyteamtag (`/Game/BPs/BaseCharacterBP.EnemyTeamTag` _weaponowner))
  (`/Engine/EditorBlueprintResources/StandardMacros.IsValid` _weaponowner
    (:`Is Valid`
      (if (`/Game/BPs/BaseCharacterBP.IsAttacking` _weaponowner)
        (if (`/Game/BPs/BaseCharacterBP.HeavyAttack` _weaponowner)
          ;[1 1 1] Heavy Attack
          (message `/Game/BPs/Interfaces/DamagableInterface.getDamaged` OtherActor (`self.HeavyAttackDamage`) (`self.DamageType`) _enemyteamtag (`/Game/BPs/MacroFunctionLibraries/AvastYeActorMacros.DirectionalKnockback` OtherActor _weaponowner (`self.HeavyKnockBack`) (`self.HeavyKnockUp`)) (`self.WeaponStunDuration`) _weaponowner OverlappedComponent)
          (`GameplayStatics.SpawnEmitterAtLocation` (`self.HitParticle`) _returnvalue (struct) (1.5 1.5 1.5))
          (else
            ;[1 1 1] Light Attack
            (message `/Game/BPs/Interfaces/DamagableInterface.getDamaged` OtherActor (`self.LightAttackDamage`) (`self.DamageType`) _enemyteamtag (`/Game/BPs/MacroFunctionLibraries/AvastYeActorMacros.DirectionalKnockback` OtherActor _weaponowner (`self.LightKnockBack`) (`self.LightKnockUp`)) (* (`self.WeaponStunDuration`) 0.6) _weaponowner OverlappedComponent)
            (`GameplayStatics.SpawnEmitterAtLocation` (`self.HitParticle`) _returnvalue)))))))

(fn `UserConstructionScript`
  (`parent.UserConstructionScript`))