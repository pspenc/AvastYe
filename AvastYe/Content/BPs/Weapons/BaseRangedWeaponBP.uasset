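; Base ranged weapon Blueprint that spawns projectiles of its BulletType when fired.
; Fire launches from the weapon's location toward TargetPoint, or along the weapon's rotation if the point is zero, passing the owner as Shooter with its EnemyTeamTag.
; BulletSpread offers random pitch and yaw jitter but is unused in these graphs.
; AltFire and Reload are empty stubs.
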(event `Fire`
  (params (TargetPoint :type "Vector Structure"))
  (bind _returnvalue (`self.K2_GetActorLocation`))
  (bind _weaponowner (`self.WeaponOwner`))
  (bind _weaponowner_2 (`self.WeaponOwner`))
  (if (== TargetPoint (0.0 0.0 0.0))
    (`|SpawnActorFromClass` (`self.BulletType`) (`KismetMathLibrary.MakeTransform` (`self.K2_GetActorLocation`) (`self.K2_GetActorRotation`)) "AdjustIfPossibleButAlwaysSpawn" "OverrideRootScale" null (`/Game/BPs/BaseCharacterBP.EnemyTeamTag` _weaponowner) _weaponowner null)
    (else
      (`|SpawnActorFromClass` (`self.BulletType`) (`KismetMathLibrary.MakeTransform` _returnvalue (`KismetMathLibrary.FindLookAtRotation` _returnvalue TargetPoint)) "AdjustIfPossibleButAlwaysSpawn" "OverrideRootScale" null (`/Game/BPs/BaseCharacterBP.EnemyTeamTag` _weaponowner_2) _weaponowner_2 null))))

(event `AltFire`
  (params (TargetPoint :type "Vector Structure"))
  (if (== TargetPoint (0.0 0.0 0.0))
    _))

(event `Reload`)

(fn `BulletSpread`
  (params (Spread :type "Float (double-precision)") (`In Transform` :type "Transform Structure"))
  (returns (NewTransform :type "Transform Structure"))
  (bind _returnvalue (* Spread -1.0))
  (return (`KismetMathLibrary.MakeTransform` (.location `In Transform`) (`KismetMathLibrary.MakeRotator` (.roll (.rotation `In Transform`)) (+ (.pitch (.rotation `In Transform`)) (`KismetMathLibrary.RandomFloatInRange` _returnvalue Spread)) (+ (.yaw (.rotation `In Transform`)) (`KismetMathLibrary.RandomFloatInRange` _returnvalue Spread))) (.scale `In Transform`))))

(fn `UserConstructionScript`
  (`parent.UserConstructionScript`))