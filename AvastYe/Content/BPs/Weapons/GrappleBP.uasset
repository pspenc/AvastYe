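; Grappling hook weapon that pulls the player to targets, or optionally pulls tagged enemies to the player.
; Without a supplied target, Targeting runs widening sphere traces along the camera.
; A looping timer drives GrappleLoop, extending the rope, then repeatedly calling LaunchCharacter with time-eased, input-steered swing velocity until within range.
; Grappled enemies are stunned, and reaching one without pulling deals damage, knocks it back and bounces the player away.
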(event Custom|Grapple
  (params (PullEnemy :type Boolean) (TargetActor :type Actor%20Object%20Reference))
  (Variables|Default|SetPullEnemy PullEnemy)
  (if (Variables|Default|GetGrappling) ; Check if Already Grappling
    (CallFunction|ResetGrapple) ; Reset Grapple
    (Utilities|Time|ClearTimerbyFunctionName 0 "GrappleLoop") ; Stop Grapple Loop
    (else
      (Variables|Default|SetGrappling true)
      (Utilities|IsValid TargetActor
        (:Is%20Valid
          (Variables|Default|SetGrappleTarget TargetActor) ; Mark GrappleTarget as Null
          (bind _returnvalue (GameplayTags|HasMatchingGameplayTag(Message) (Variables|Default|GetGrappleTarget) "(TagName=\"Team.BadGuy\")" :!label _label))
          (Variables|Default|SetEnemyTarget _returnvalue)
          (Variables|Default|SetFoundTarget false) ; Reset FoundTarget
          (Utilities|Time|SetTimerbyFunctionName 0 "GrappleLoop" 0.01 true) ; Begin Grapple Loop
          (Input|DisableInput (Game|GetPlayerController 0)))
        (:Is%20Not%20Valid
          (bind _successful (CallFunction|Targeting)) ; Check for Interactive Objects & Enemies
          (if _successful
            (goto _label)
            (else
              (Variables|Default|SetGrappleTarget 0) ; Mark GrappleTarget as Null
            )))))))

(event Custom|ResetGrapple
  (bind _grappleline (Variables|Default|GetGrappleLine))
  ;[1 1 1] End Grapple
  (Variables|Default|SetGrappling false)
  (Rendering|SetVisibility _grappleline false true)
  (Transformation|SetWorldLocation _grappleline (Transformation|GetActorLocation) false false) ; This causes weird bug where shooting in some directions mirrors the look direction
)

(event Input|AxisEvents|InputAxisMoveRight
  (params (AxisValue :type Float%20%28single-precision%29))
  (Variables|Default|SetCustomMoveRight AxisValue))

(event Input|AxisEvents|InputAxisMoveForward
  (params (AxisValue :type Float%20%28single-precision%29))
  (Variables|Default|SetCustomMoveForward AxisValue))

(fn ConstructionScript)

(fn GrappleLoop
  (bind _character (Variables|Default|GetCharacter))
  (bind _character_2 (Variables|Default|GetCharacter))
  (if (Variables|Default|GetGrappleLanded) ; Check Whether Grapple has Landed
    (if (Variables|Default|GetEnemyTarget) ; Ceck for Enemy Target
      (Class|DamagableInterface|GetDamaged(Message) (Variables|Default|GetGrappleTarget) 0.0 "NewEnumerator0" "(TagName=\"Team.BadGuy\")" "0, 0, 0" 3.0 (stale _ascaptain_character)) ; Stun Grappled Enemy
      (if (Variables|Default|GetPullEnemy)
        (if (Variables|Default|GetGrappleRetracted)
          (Variables|Default|SetGrappleLanded false) ; Reset GrappleLanded
          (Variables|Default|SetGrappleRetracted false) ; Reset PlayerLanded
          (Variables|Default|SetPullEnemy false) ; Reset Pull Enemy
          (CallFunction|ResetGrapple :!label _label) ; Reset Grapple
          (Utilities|Time|ClearTimerbyFunctionName 0 "GrappleLoop") ; Stop Grapple Loop
          (else
            (CallFunction|MoveEnemy)
            (CallFunction|UpdateRope)))
        (else
          (if (Variables|Default|GetGrappleRetracted) :!label _label_2
            (Variables|Default|SetGrappleLanded false) ; Reset GrappleLanded
            (Variables|Default|SetGrappleRetracted false) ; Reset PlayerLanded
            (if (Variables|Default|GetEnemyTarget) ; Damage Approached Enemies
              (bind _ascaptain_character (Utilities|Casting|CastToCaptainCharacter _character))
              (Class|DamagableInterface|GetDamaged(Message) (Variables|Default|GetGrappleTarget) 2e+01 "NewEnumerator3" "(TagName=\"Team.BadGuy\")" (Utilities|MakeForceVector (Transformation|GetActorForwardVector _character) 2e+02 5e+02) 0.0 _ascaptain_character)
              (Character|LaunchCharacter _character_2 (Utilities|MakeForceVector (* (Transformation|GetActorForwardVector _character_2) -1) 2e+02 5e+02) true true)
              (goto _label)
              (else
                (goto _label)))
            (else
              (CallFunction|MoveCharacter false) ; Move Character to Intended Target
              (CallFunction|UpdateRope) ; Update Rope
            ))))
      (else
        (goto _label_2)))
    (else
      (CallFunction|MoveRope) ; Move Rope to Intended Target
    )))

(fn MoveRope
  (bind _grappleline (Variables|Default|GetGrappleLine))
  (bind _grappletarget (Variables|Default|GetGrappleTarget))
  (bind _returnvalue (Transformation|GetWorldLocation _grappleline))
  (bind _returnvalue_2 (Transformation|GetActorLocation _grappletarget))
  (Utilities|IsValid _grappletarget
    (:Is%20Valid
      (Rendering|SetVisibility _grappleline true true) ; Make the Grapple Visible
      (if (<= (Math|Vector|VectorLength (- _returnvalue _returnvalue_2)) 1e+02) ; Check if GrappleLine has Landed
        (Variables|Default|SetGrappleLanded true)
        (Variables|Default|SetGrappleTime (Utilities|Time|GetGameTimeinSeconds)) ; Store Time of Landed Grapple
        (Variables|Default|SetGrappleDist (Math|Vector|VectorLength (- (Transformation|GetActorLocation (Variables|Default|GetGrappleTarget)) (Transformation|GetActorLocation (Variables|Default|GetCharacter))))) ; Get the Distance Between Player and Target
        (else
          (Transformation|SetWorldLocation (Variables|Default|GetGrappleLine) (Math|Interpolation|VInterpTo _returnvalue _returnvalue_2 (Utilities|Time|GetWorldDeltaSeconds) (Variables|Default|GetLaunchSpeed)) false false)
          (Variables|Default|SetGrappleLanded false))))))

(fn MoveCharacter
  (params (NewParam :type Boolean))
  (bind _returnvalue (Utilities|Time|GetGameTimeinSeconds))
  (bind _returnvalue_2 (Utilities|Time|GetWorldDeltaSeconds))
  (bind _returnvalue_3 (Input|AxisValues|GetMoveRight))
  (bind _character (Variables|Default|GetCharacter))
  (bind _grappletime (Variables|Default|GetGrappleTime))
  (bind _grappledist (Variables|Default|GetGrappleDist))
  (bind _movespeed (Variables|Default|GetMoveSpeed))
  (bind _character_2 (Variables|Default|GetCharacter))
  (bind _grappletarget (Variables|Default|GetGrappleTarget))
  (bind _returnvalue_4 (- _returnvalue _grappletime))
  (bind _returnvalue_5 (Transformation|GetActorLocation _character))
  (bind _returnvalue_6 (Transformation|GetActorLocation _grappletarget))
  (bind _returnvalue_7 (* 1.0 _returnvalue_3))
  (bind _returnvalue_8 (* _returnvalue_2 _movespeed))
  (bind _returnvalue_9 (- _returnvalue_6 _returnvalue_5))
  (bind _returnvalue_10 (* _returnvalue_4 -1.0))
  (bind _returnvalue_11 (Math|Vector|VectorLength _returnvalue_9))
  (bind _returnvalue_12 (Math|Vector|CrossProduct "0, 0,1.000000" _returnvalue_9))
  (bind _returnvalue_13 (* _returnvalue_10 8.0))
  (bind _returnvalue_14 (* _returnvalue_12 _returnvalue_7))
  (bind _returnvalue_15 (- _returnvalue_13 1.0))
  (bind _returnvalue_16 (- _grappledist _returnvalue_11))
  (bind _returnvalue_17 (/ 1.0 _returnvalue_15))
  (bind _returnvalue_18 (/ _returnvalue_16 _grappledist))
  (bind _returnvalue_19 (Math|Float|Sqrt _returnvalue_18))
  (bind _returnvalue_20 (+ _returnvalue_17 1.0))
  (bind _returnvalue_21 (* _returnvalue_14 _returnvalue_19))
  (bind _returnvalue_22 (+ _returnvalue_21 _returnvalue_9))
  (bind _returnvalue_23 (Math|Vector|Normalize _returnvalue_22))
  (bind _returnvalue_24 (* _returnvalue_23 _returnvalue_20))
  (bind _returnvalue_25 (* _returnvalue_24 1e+03))
  (bind _returnvalue_26 (* _returnvalue_25 _returnvalue_8))
  (Utilities|IsValid _grappletarget
    (:Is%20Valid
      (if (>= _returnvalue_11 2e+02) ; Check Distance to Final Grapple Point
        (if (Variables|Default|GetEnemyTarget) ; Slow Down if Not Attacking
          (Character|LaunchCharacter _character_2 _returnvalue_26 true true) ; Movement when Attacking
          (else
            (Character|LaunchCharacter _character_2 (* _returnvalue_26 (Math|Float|Clamp(Float) (/ (Math|Float|Clamp(Float) (- _returnvalue_11 7e+01) 0.0 1e+06) 1e+03))) true true) ; Movement When Grappling
          ))
        (else
          (Variables|Default|SetGrappleRetracted true))))
    (:Is%20Not%20Valid)))

(fn UpdateRope
  (bind _grappleline (Variables|Default|GetGrappleLine))
  (bind _grappletarget (Variables|Default|GetGrappleTarget))
  (bind _returnvalue (Transformation|GetActorLocation _grappletarget))
  (Transformation|SetWorldLocationAndRotation _grappleline (Math|Interpolation|VInterpTo (Transformation|GetWorldLocation _grappleline) _returnvalue (Utilities|Time|GetWorldDeltaSeconds) 2.5e+02) (Math|Rotator|FindLookatRotation (Transformation|GetActorLocation (Variables|Default|GetCharacter)) _returnvalue) false false))

(fn MoveEnemy
  (bind _character (Variables|Default|GetCharacter))
  (bind _grappledist (Variables|Default|GetGrappleDist))
  (bind _grappletarget (Variables|Default|GetGrappleTarget))
  (bind _returnvalue (Transformation|GetActorLocation _character))
  (bind _returnvalue_2 (Transformation|GetActorLocation _grappletarget))
  (bind _returnvalue_3 (- _returnvalue _returnvalue_2))
  (bind _returnvalue_4 (Math|Vector|VectorLength _returnvalue_3))
  (Utilities|IsValid _grappletarget
    (:Is%20Valid
      (if (>= _returnvalue_4 2e+02) ; Check Distance to Final Grapple Point
        (bind _ascharacter (Utilities|Casting|CastToCharacter (Variables|Default|GetGrappleTarget)))
        (Character|LaunchCharacter _ascharacter (* (* (* (* (Math|Vector|Normalize (+ (* (* (Math|Vector|CrossProduct "0, 0,1.000000" _returnvalue_3) (* 1.0 (Input|AxisValues|GetMoveRight))) (Math|Float|Sqrt (/ (- _grappledist _returnvalue_4) _grappledist))) _returnvalue_3)) (+ (/ 1.0 (- (* (* (- (Utilities|Time|GetGameTimeinSeconds) (Variables|Default|GetGrappleTime)) -1.0) 8.0) 1.0)) 1.0)) 1e+03) (* (Utilities|Time|GetWorldDeltaSeconds) (* (Variables|Default|GetMoveSpeed) 2.0))) (Math|Float|Clamp(Float) (/ (Math|Float|Clamp(Float) (- _returnvalue_4 7e+01) 0.0 1e+06) 1.2e+03))) true true) ; Movement When Grappling
        (else
          (Variables|Default|SetGrappleRetracted true))))
    (:Is%20Not%20Valid)))

(fn Targeting
  (bind _character (Variables|Default|GetCharacter))
  (bind _follow_camera (Variables|Default|GetFollow%20Camera))
  (bind _returnvalue (Transformation|GetActorLocation _character))
  (bind _returnvalue_2 (Math|Vector|GetForwardVector _follow_camera))
  (bind _index (Utilities|FlowControl|ForLoopwithBreak 0 3 :!label _label) ; Loop through progressively larger search areas
    (:LoopBody
      ;[1 1 1] Trace Debug Color
      (switch int _index
        (:0
          (Variables|Default|SetTraceDebugColor "(R=1.000000,G=0.000000,B=0.000000,A=1.000000)"))
        (:1
          (Variables|Default|SetTraceDebugColor "(R=1.000000,G=0.837630,B=0.000000,A=1.000000)"))
        (:2
          (Variables|Default|SetTraceDebugColor "(R=0.178136,G=1.000000,B=0.000000,A=1.000000)"))
        (:3
          (Variables|Default|SetTraceDebugColor "(R=0.000000,G=0.020782,B=1.000000,A=1.000000)")))
      (if (<= _index 0)
        (Variables|Default|SetTargetingRadius 1e+01)
        (else
          (Variables|Default|SetTargetingRadius (* (Math|Float|Power 2.0 (Math|Conversions|ToFloat(Integer) _index)) 1e+02))))
      (bind (_outhits _returnvalue_3) (Collision|MultiSphereTraceForObjects (+ _returnvalue (* _returnvalue_2 5e+02)) (+ (* _returnvalue_2 5e+03) _returnvalue) (Variables|Default|GetTargetingRadius) (Utilities|Array|MakeArray "ObjectTypeQuery8" "ObjectTypeQuery11") false 0 "None" true (Variables|Default|GetTraceDebugColor) (Variables|Default|GetTraceDebugColor)))
      (if _returnvalue_3
        (bind _array_element (Utilities|Array|ForEachLoopwithBreak _outhits :!label _label_2)
          (:LoopBody
            (Variables|Default|SetGrappleTarget (.HitActor (Collision|BreakHitResult _array_element)))
            (Variables|Default|SetFoundTarget true)
            (goto _label_2 Break))
          (:Completed
            (goto _label Break)))))
    (:Completed
      (return (Variables|Default|GetFoundTarget)))))