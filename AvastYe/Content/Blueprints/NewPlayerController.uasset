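; Player controller that switches the player between the third-person character and three ant types: carpenter, fire and bull.
; Hard-coded number key presses each look up all actors of one class and possess the first one found.
; There is no check that an instance exists before possessing, and BeginPlay and Tick are unused.
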(event `Key|Zero`
  (params (Key :type "Key Structure"))
  (:`Pressed`
    (bind _outactors (`GameplayStatics.GetAllActorsOfClass` "/Game/BPs/ThirdPersonCharacter.ThirdPersonCharacter_C"))
    (`self.Possess` (`|GetArrayItem` _outactors))))

(event `Key|Seven`
  (params (Key :type "Key Structure"))
  (:`Pressed`
    (bind _outactors (`GameplayStatics.GetAllActorsOfClass` "/Game/BPs/AI/CarpenterAnt.CarpenterAnt_C"))
    (`self.Possess` (`|GetArrayItem` _outactors))))

(event `Key|Eight`
  (params (Key :type "Key Structure"))
  (:`Pressed`
    (bind _outactors (`GameplayStatics.GetAllActorsOfClass` "/Game/BPs/AI/FireAnt.FireAnt_C"))
    (`self.Possess` (`|GetArrayItem` _outactors))))

(event `Key|Nine`
  (params (Key :type "Key Structure"))
  (:`Pressed`
    (bind _outactors (`GameplayStatics.GetAllActorsOfClass` "/Game/BPs/AI/BullAnt.BullAnt_C"))
    (`self.Possess` (`|GetArrayItem` _outactors))))

(fn `UserConstructionScript`)