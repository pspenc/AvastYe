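; Base AI pawn Blueprint that connects inherited combat reactions (damage, hitstun, status effects) to the AI's decision-making.
; Hitstun and stun clearing copy AbleToAct into the blackboard, and an ended ability clears the blackboard's ability lock.
; Damage and status overrides call the parent, then notify the AI controller of damage taken (except one attack type) or catching fire.
; An unconnected sphere-trace damage chain remains in the event graph.
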(event `self.ApplyHitstun`
  (params (Hitstun :type "Float (single-precision)"))
  (bind _returnvalue (`AIBlueprintHelperLibrary.GetBlackboard` self))
  (`parent.ApplyHitstun` Hitstun)
  (`/Engine/EditorBlueprintResources/StandardMacros.IsValid` _returnvalue
    (:`Is Valid`
      (`BlackboardComponent.SetValueAsBool` _returnvalue (`self.AbleToActBBKey`) (`self.AbleToAct`)))))

(event `self.ClearStunned`
  (bind _returnvalue (`AIBlueprintHelperLibrary.GetBlackboard` self))
  (`parent.ClearStunned`)
  (`/Engine/EditorBlueprintResources/StandardMacros.IsValid` _returnvalue
    (:`Is Valid`
      (`BlackboardComponent.SetValueAsBool` _returnvalue (`self.AbleToActBBKey`) (`self.AbleToAct`)))))

(event `self.AbilityEnded`
  (`BlackboardComponent.SetValueAsBool` (`AIBlueprintHelperLibrary.GetBlackboard` self) (`self.AbilityLockBBKey`) false))

(fn `ApplyDamage`
  (params (Damage :type "Float (double-precision)") (Hitstun :type "Float (double-precision)") (ForceVector :type "Vector Structure") (`Damage Type` :type "/Game/RebuildBPs/Enumerations/DamageType Enum" :default "NewEnumerator0") (`Attack Type` :type "/Game/RebuildBPs/Enumerations/AttackType Enum" :default "NewEnumerator0") (Attacker :type "/Game/RebuildBPs/BaseCharacterRBP Object Reference") (`Hit Component` :type "PrimitiveComponent Object Reference") (`Team to Damage` :type "GameplayTag Structure"))
  (returns (Died :type Boolean) (DamageTaken :type Boolean))
  (bind (_died _damagetaken) (`parent.ApplyDamage` Damage Hitstun ForceVector `Damage Type` `Attack Type` Attacker `Hit Component` `Team to Damage`))
  (if (and (`|EnumInequality` `Attack Type` "NewEnumerator4") _damagetaken)
    (message `/Game/RebuildBPs/Interfaces/AICommunicationInterfaceR.PawnGotDamaged` (`AIBlueprintHelperLibrary.GetAIController` self)))
  (return _died _damagetaken))

(fn `ApplyStatusEffects`
  (params (`Attack Type` :type "/Game/RebuildBPs/Enumerations/AttackType Enum" :default "NewEnumerator0") (`Status Effect` :type "/Game/RebuildBPs/StatusEffects/BaseStatusEffect Class Reference") (Attacker :type "/Game/RebuildBPs/BaseCharacterRBP Object Reference"))
  (returns (`Effect Applied` :type Boolean))
  (bind _effect_applied (`parent.ApplyStatusEffects` `Attack Type` `Status Effect` Attacker))
  (if (and _effect_applied (== `Status Effect` "/Game/RebuildBPs/StatusEffects/OnFire.OnFire_C"))
    (message `/Game/RebuildBPs/Interfaces/AICommunicationInterfaceR.PawnOnFire` (`AIBlueprintHelperLibrary.GetAIController` self)))
  (return _effect_applied))

(fn `UserConstructionScript`
  (`parent.UserConstructionScript`))