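; Base enemy character for AI foes, handling combat state, health UI and death drops.
; A Director tracks its target switches, attack ends and death, while blackboard keys mirror target and attack state.
; Armor reduces damage and hitstun, blocks burning, and breaks in two stages from captain damage or at once from one damage type.
; Captain hits draw aggro and briefly tag the enemy to lower its priority for crew targeting.
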(event `self.ReceiveBeginPlay`
  (bind _aggrdeviation (`self.AggrDeviation`))
  (bind _damageresistances (`self.DamageResistances`))
  (bind _armordamagemultiplier (`self.ArmorDamageMultiplier`))
  ;[1 1 1] Begin Play/Modifier setup
  (`parent.ReceiveBeginPlay`)
  (set `self.Health` (* (`self.Health`) (`self.StartingHealthModifier`)))
  (set `self.Aggressiveness` (+ (`self.Aggressiveness`) (`KismetMathLibrary.RandomFloatInRange` (* _aggrdeviation -1.0) _aggrdeviation)))
  (if (`self.Armored`)
    (`BlueprintMapLibrary.Map_Add` _damageresistances "" _armordamagemultiplier)
    (`BlueprintMapLibrary.Map_Add` _damageresistances "NewEnumerator2" _armordamagemultiplier)
    (`BlueprintMapLibrary.Map_Add` _damageresistances "NewEnumerator3" _armordamagemultiplier))
  (`self.InitHealthBar`)
  ;[1 1 1] FOR DEBUGGING
  (if (`self.NameVisible`)
    (`self.MakeTextFavceCameraRecursive`)))

(event `MakeTextFavceCameraRecursive`
  ;[1 1 1] FOR DEBUGGING
  (`self.MakeTextFaceCamera`)
  (`KismetSystemLibrary.K2_SetTimerDelegate` (delegate `MakeTextFavceCameraRecursive`) 0.2))

(event `Initialize`
  (if (`self.UsableWings`)
    (`BlackboardComponent.SetValueAsBool` (`AIBlueprintHelperLibrary.GetBlackboard` null) (`self.UsableWingsBBKey`) (`self.UsableWings`))))

(event `MakeTextFaceCamera`
  (bind _textrender (`self.TextRender`))
  ;[1 1 1] FOR DEBUGGING
  (`SceneComponent.K2_SetWorldRotation` _textrender (`KismetMathLibrary.MakeRotFromX` (- (`SceneComponent.K2_GetComponentLocation` (`/Game/RebuildBPs/CaptainCharacterRBP.FollowCamera` (`/Game/RebuildBPs/AvastYeRGameMode.Captain` (cast `/Game/RebuildBPs/AvastYeRGameMode` (`GameplayStatics.GetGameMode`) :!pure true)))) (`SceneComponent.K2_GetComponentLocation` _textrender))) false false))

(event `self.IsTargetOfAbility`)

(event `EndAttackBroadcast`
  (bind _director (`self.Director`))
  ;[1 1 1] End Attack Broadcast
  (`/Engine/EditorBlueprintResources/StandardMacros.IsValid` _director
    (:`Is Valid`
      (`BlackboardComponent.SetValueAsBool` (`AIBlueprintHelperLibrary.GetBlackboard` null) (`self.AttackingBBKey`) false)
      (`/Game/RebuildBPs/AI/EnemyAIDirectorR.UnitEndAttackingTarget` _director (`self.CurrentTarget`))
      (`KismetSystemLibrary.Delay` 0.2)
      (set `self.ToldToAttack` false))))

(event `AlertDirectorOfDeath`
  (bind _director (`self.Director`))
  ;[1 1 1] Alert Director of Death
  (`/Engine/EditorBlueprintResources/StandardMacros.IsValid` _director
    (:`Is Valid`
      (`/Game/RebuildBPs/AI/EnemyAIDirectorR.UnitHasDied` _director self))))

(event `InitHealthBar`
  ;[1 1 1] Init Health
  (bind _asrenemy_ui (cast `/Game/RebuildBPs/UI/REnemyUI` (`WidgetComponent.GetUserWidgetObject` (`self.EnemyUI`))))
  (set `self.EnemyUIReference` _asrenemy_ui)
  (set `/Game/RebuildBPs/UI/REnemyUI.Enemy` self _asrenemy_ui))

(event `ShowHealth`
  (bind _enemyuireference (`self.EnemyUIReference`))
  ;[1 1 1] Init Health
  (set `/Game/RebuildBPs/UI/REnemyUI.Size` (`self.HealthBarSize`) _enemyuireference)
  (`/Game/RebuildBPs/UI/REnemyUI.ChangeColor` _enemyuireference (struct :`R` 1.0 :`B` 0.6 :`A` 1.0))
  (if (`self.Armored`)
    (`/Game/RebuildBPs/UI/REnemyUI.EnableGuard` _enemyuireference))
  (`/Game/RebuildBPs/UI/REnemyUI.ShowHealthBar` _enemyuireference))

(event `ChangeTarget`
  (params (NewTarget :type "/Game/RebuildBPs/BaseCharacterRBP Object Reference"))
  (bind _currenttarget (`self.CurrentTarget`))
  (bind _director (`self.Director`))
  ;[1 1 1] Change Target
  (if (!= NewTarget _currenttarget)
    (`/Engine/EditorBlueprintResources/StandardMacros.IsValid` _director
      (:`Is Valid`
        (`/Game/RebuildBPs/AI/EnemyAIDirectorR.UnitSwitchingTargets` _director self NewTarget _currenttarget)))))

(event `Set Target`
  (params (Target :type "/Game/RebuildBPs/BaseCharacterRBP Object Reference"))
  (bind _returnvalue (`AIBlueprintHelperLibrary.GetBlackboard` self))
  ;[1 1 1] Set Target
  (bind _output_get (set `self.CurrentTarget` Target))
  (`/Engine/EditorBlueprintResources/StandardMacros.IsValid` _returnvalue
    (:`Is Valid`
      (`BlackboardComponent.SetValueAsObject` _returnvalue (`self.TargetEnemyBBKey`) _output_get))))

(event `Attack Target`
  ;[1 1 1] Attack Target
  (bind _output_get (set `self.ToldToAttack` true))
  (`BlackboardComponent.SetValueAsBool` (`AIBlueprintHelperLibrary.GetBlackboard` null) (`self.AttackingBBKey`) _output_get))

(event `self.BecomeFollowUpTarget`
  (params (Captain :type "/Game/RebuildBPs/CaptainCharacterRBP Object Reference"))
  ;[1 1 1] Become/Clear Follow Up Target
  (`/Game/RebuildBPs/UI/REnemyUI.On` (`self.EnemyUIReference`) Captain)
  (set `self.IsFollowupTarget` true))

(event `self.ClearFollowUpTarget`
  ;[1 1 1] Become/Clear Follow Up Target
  (`/Game/RebuildBPs/UI/REnemyUI.Off` (`self.EnemyUIReference`))
  (set `self.IsFollowupTarget` false))

(event `self.GetDamaged`
  (params (Damage :type "Float (single-precision)") (Hitstun :type "Float (single-precision)") (ForceVector :type "Vector Structure") (`Damage Type` :type "/Game/RebuildBPs/Enumerations/DamageType Enum" :default "NewEnumerator0") (`Attack Type` :type "/Game/RebuildBPs/Enumerations/AttackType Enum" :default "NewEnumerator0") (Attacker :type "/Game/RebuildBPs/BaseCharacterRBP Object Reference") (`Hit Component` :type "PrimitiveComponent Object Reference") (`Enemy Team` :type "GameplayTag Structure") (`Status Effect` :type "/Game/RebuildBPs/StatusEffects/BaseStatusEffect Class Reference"))
  ;[1 1 1] Get Damaged
  (if (== (`GameplayStatics.GetObjectClass` Attacker) "/Game/RebuildBPs/CaptainCharacterRBP.CaptainCharacterRBP_C")
    (`self.BecomeCaptain'sTarget`)
    (`self.ChangeTarget` Attacker)
    (if (`self.Armored`)
      (`self.ProcessArmor Damage` Damage)))
  (`parent.GetDamaged` Damage Hitstun ForceVector `Damage Type` `Attack Type` Attacker `Hit Component` `Enemy Team` `Status Effect`))

(event `self.Get Targeted`
  (bind _enemyuireference (`self.EnemyUIReference`))
  ;[1 1 1] Show/Hide Targeting Indicator
  (`/Engine/EditorBlueprintResources/StandardMacros.IsValid` _enemyuireference
    (:`Is Valid`
      (`/Game/RebuildBPs/UI/REnemyUI.TargetedON` _enemyuireference))))

(event `self.PerfectWindowStartNotify`
  (bind _currenttarget (`self.CurrentTarget`))
  (`/Engine/EditorBlueprintResources/StandardMacros.IsValid` _currenttarget
    (:`Is Valid`
      (`self.StartPerfectWindow` _currenttarget self))))

(event `self.Get Un-Targeted`
  (bind _enemyuireference (`self.EnemyUIReference`))
  ;[1 1 1] Show/Hide Targeting Indicator
  (`/Engine/EditorBlueprintResources/StandardMacros.IsValid` _enemyuireference
    (:`Is Valid`
      (`/Game/RebuildBPs/UI/REnemyUI.TargetedOFF` _enemyuireference))))

(event `self.PerfectWindownStopNotify`
  (bind _currenttarget (`self.CurrentTarget`))
  (`/Engine/EditorBlueprintResources/StandardMacros.IsValid` _currenttarget
    (:`Is Valid`
      (`self.EndPerfectWindow` _currenttarget))))

(event `BecomeCaptain'sTarget`
  ;[1 1 1] Become Captain's Target (to lower targeting priority for crew members)
  (`BlueprintGameplayTagLibrary.AddGameplayTag` (`self.GameplayTags`) (struct :`TagName` "TargetingInfo.CaptainsTarget"))
  (`KismetSystemLibrary.K2_SetTimerDelegate` (delegate `NoLongerCaptain'sTarget`) 3.0))

(event `NoLongerCaptain'sTarget`
  ;[1 1 1] Become Captain's Target (to lower targeting priority for crew members)
  (`BlueprintGameplayTagLibrary.RemoveGameplayTag` (`self.GameplayTags`) (struct :`TagName` "TargetingInfo.CaptainsTarget")))

(event `Break Armor`
  (params (PiecesToBreak :type Integer))
  (bind _returnvalue (`self.K2_GetActorLocation`))
  (bind _returnvalue_2 (`self.K2_GetActorLocation`))
  (bind _damageresistances (`self.DamageResistances`))
  (bind _temp_armor1 (`self.temp_armor1`))
  (bind _damageresistances_2 (`self.DamageResistances`))
  (bind _returnvalue_3 (* (`self.ArmorDamageMultiplier`) 2.0))
  ;[1 1 1] Break Armor
  (if (>= PiecesToBreak 2)
    (set `self.Armored` false :!label _label)
    (`SceneComponent.SetVisibility` (`self.temp_armor`) false false)
    (`SceneComponent.SetVisibility` _temp_armor1 false false)
    (`GameplayStatics.PlaySoundAtLocation` "/Game/Assets/SoundEffects/shield_hit_01.shield_hit_01" _returnvalue_2 (struct) 1.2 0.7 0.0 null null null)
    (`GameplayStatics.SpawnEmitterAtLocation` "/Game/AdvancedMagicFX13/Particles/P_ky_impact.P_ky_impact" _returnvalue_2 (struct) (2.0 2.0 2.0))
    (`/Game/RebuildBPs/UI/REnemyUI.DisableGuard` (`self.EnemyUIReference`))
    (`BlueprintMapLibrary.Map_Add` _damageresistances_2 "" 1.0)
    (`BlueprintMapLibrary.Map_Add` _damageresistances_2 "NewEnumerator3" 1.0)
    (`BlueprintMapLibrary.Map_Add` _damageresistances_2 "NewEnumerator2" 1.0)
    (`BlackboardComponent.SetValueAsBool` (`AIBlueprintHelperLibrary.GetBlackboard` null) (`self.ArmoredBBKey`) false)
    (elif (`self.1stArmorBroken`)
      (goto _label)
      (else
        (set `self.1stArmorBroken` true)
        (`SceneComponent.SetVisibility` _temp_armor1 false false)
        (`GameplayStatics.PlaySoundAtLocation` "/Game/Assets/SoundEffects/shield_hit_01.shield_hit_01" _returnvalue (struct) 1.2 0.7 0.0 null null null)
        (`GameplayStatics.SpawnEmitterAtLocation` "/Game/AdvancedMagicFX13/Particles/P_ky_impact.P_ky_impact" _returnvalue (struct) (2.0 2.0 2.0))
        (`BlueprintMapLibrary.Map_Add` _damageresistances "" _returnvalue_3)
        (`BlueprintMapLibrary.Map_Add` _damageresistances "NewEnumerator3" _returnvalue_3)
        (`BlueprintMapLibrary.Map_Add` _damageresistances "NewEnumerator2" _returnvalue_3)))))

(event `self.Die`
  ;[1 1 1] Die
  (`self.EndAttackBroadcast`)
  (`self.AlertDirectorOfDeath`)
  (`self.DropGold`)
  (`self.DropHealthPickup`)
  (if (`self.IsFollowupTarget`)
    (`self.ClearFollowUpTarget`))
  (`KismetSystemLibrary.Delay` 0.2)
  (`parent.Die`))

(event `DropHealthPickup`
  ;[1 1 1] Drop Health Pickup
  (if (`self.ShouldDropHealthPickup`)
    (`/Engine/EditorBlueprintResources/StandardMacros.DoOnce` false
      (:`Completed`
        (`|SpawnActorFromClass` "/Game/RebuildBPs/EnvObjects/HealthPickup.HealthPickup_C" (`KismetMathLibrary.MakeTransform` (`self.K2_GetActorLocation`) (struct) (0.2 0.2 0.2)) "Undefined" "OverrideRootScale" null null)))))

(event `DropGold`
  ;[1 1 1] Drop Money
  (if (<= (`KismetMathLibrary.RandomFloatInRange` 0.0 1.0) 0.2)
    (`GameplayStatics.SpawnEmitterAtLocation` "/Game/Assets/VisualEffects/CoinEmitter/CoinMeshParticle.CoinMeshParticle" (+ (`self.K2_GetActorLocation`) (0.0 0.0 100.0)))
    (`KismetSystemLibrary.PrintString` "Coins should be droppin")
    (bind _asavast_ye_rgame_mode (cast `/Game/RebuildBPs/AvastYeRGameMode` (`GameplayStatics.GetGameMode`)))
    (`/Game/RebuildBPs/AvastYeRGameMode.IncrementGoldCount` _asavast_ye_rgame_mode (`KismetMathLibrary.RandomIntegerInRange` 5 20))
    (`GameplayStatics.SpawnEmitterAtLocation` "/Game/Assets/VisualEffects/CamilleTestFolder/P_Sparkles.P_Sparkles")
    (`/Game/RebuildBPs/AvastYeRGameMode.SaveGame` _asavast_ye_rgame_mode)))

(fn `ApplyStatusEffects`
  (params (`Attack Type` :type "/Game/RebuildBPs/Enumerations/AttackType Enum" :default "NewEnumerator0") (`Status Effect` :type "/Game/RebuildBPs/StatusEffects/BaseStatusEffect Class Reference") (Attacker :type "/Game/RebuildBPs/BaseCharacterRBP Object Reference"))
  (returns (`Effect Applied` :type Boolean))
  (if (and (`self.Armored`) (== `Status Effect` "/Game/RebuildBPs/StatusEffects/OnFire.OnFire_C"))
    (bind _effect_applied (`parent.ApplyStatusEffects` `Attack Type` null Attacker))
    (return _effect_applied)
    (else
      (bind _effect_applied_2 (`parent.ApplyStatusEffects` `Attack Type` `Status Effect` Attacker))
      (return _effect_applied_2))))

(fn `GetFollowSpot`
  (params (NumInGroup :type Integer))
  (returns (FollowLocation :type "Vector Structure"))
  (switch `int` NumInGroup
    (:`1`
      (return (`SceneComponent.K2_GetComponentLocation` (`self.Follow1`))))
    (:`2`
      (return (`SceneComponent.K2_GetComponentLocation` (`self.Follow2`))))
    (:`3`
      (return (`SceneComponent.K2_GetComponentLocation` (`self.Follow3`))))
    (:`4`
      (return (`SceneComponent.K2_GetComponentLocation` (`self.Follow4`))))
    (:`5`
      (return (`SceneComponent.K2_GetComponentLocation` (`self.Follow5`))))))

(fn `ProcessArmor Damage`
  (params (Damage :type "Float (double-precision)"))
  (locals (StartingArmorHealth :type "Float (double-precision)"))
  (bind _armorhealth (`self.ArmorHealth`))
  (set `local.StartingArmorHealth` _armorhealth)
  (set `self.ArmorHealth` (- _armorhealth Damage))
  (if (and (>= (`local.StartingArmorHealth`) 300.0) (< (`self.ArmorHealth`) 300.0))
    (set `self.ShouldBreakArmorPiece` true :!label _label)
    (elif (and (>= (`local.StartingArmorHealth`) 1.0) (< (`self.ArmorHealth`) 1.0))
      (goto _label)
      (else
        (set `self.ShouldBreakArmorPiece` false)))))

(fn `ProcessDamageModifications`
  (params (`Base Damage` :type "Float (double-precision)") (`Base Hitstun` :type "Float (double-precision)") (ForceVector :type "Vector Structure") (`Damage Type` :type "/Game/RebuildBPs/Enumerations/DamageType Enum" :default "NewEnumerator0") (`Attack Type` :type "/Game/RebuildBPs/Enumerations/AttackType Enum" :default "NewEnumerator0") (TeamToDamage :type "GameplayTag Structure") (Attacker :type "/Game/RebuildBPs/BaseCharacterRBP Object Reference"))
  (returns (`New Damage` :type "Float (double-precision)") (`New Hitstun` :type "Float (double-precision)") (`New ForceVector` :type "Vector Structure") (`Entirely Negated` :type Boolean))
  (if (and (`|EnumEquality` `Damage Type` "NewEnumerator1") (`self.Armored`))
    (`self.Break Armor` 2)
    (set `self.ArmorHealth` 0.0)
    (elif (`self.Armored`)
      (if (`self.ShouldBreakArmorPiece`)
        (set `self.ShouldBreakArmorPiece` false)
        (`self.Break Armor` 1))
      (bind (_new_damage _new_hitstun _new_forcevector _entirely_negated) (`parent.ProcessDamageModifications` `Base Damage` (- `Base Hitstun` (`self.ArmorHitstunReduction`)) (0.0 0.0 0.0) `Damage Type` `Attack Type` TeamToDamage null))
      (return _new_damage _new_hitstun _new_forcevector _entirely_negated)
      (else
        _)))
  (bind (_new_damage_2 _new_hitstun_2 _new_forcevector_2 _entirely_negated_2) (`parent.ProcessDamageModifications` `Base Damage` `Base Hitstun` ForceVector `Damage Type` `Attack Type` TeamToDamage null))
  (return _new_damage_2 _new_hitstun_2 _new_forcevector_2 _entirely_negated_2))

(fn `UserConstructionScript`
  (bind _textrender (`self.TextRender`))
  (bind _armored (`self.Armored`))
  (`parent.UserConstructionScript`)
  (`SceneComponent.SetVisibility` (`self.temp_armor`) _armored false)
  (`SceneComponent.SetVisibility` (`self.temp_armor1`) _armored false)
  (set `self.InitialLocation` (`self.K2_GetActorLocation` self))
  ;[1 1 1] FOR DEBUGGING
  (if (`self.NameVisible`)
    (`TextRenderComponent.K2_SetText` _textrender (`KismetTextLibrary.Conv_StringToText` (`KismetSystemLibrary.GetDisplayName` self)))
    (`SceneComponent.SetVisibility` _textrender true false)
    (`self.MakeTextFaceCamera`)))