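; Base crewmember character that exposes the ability casts for the Captain's AI crew, including combo follow-ups.
; On BeginPlay it caches the player pawn as the Captain.
; Tap and hold events pass a target actor and location to CastAbility with the matching ability variable.
; Knockup and AOE follow-up events, each in tap and hold versions, switch on who set up the combo (Captain, Bull, Fire or Witch) to choose the ability.
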(event `self.ReceiveBeginPlay`
  (`parent.ReceiveBeginPlay`)
  (bind _ascaptain_character_rbp (cast `/Game/RebuildBPs/CaptainCharacterRBP` (`GameplayStatics.GetPlayerPawn` 0)))
  (set `self.Captain` _ascaptain_character_rbp))

(event `Cast Tap Ability`
  (params (`Target Actor` :type "Actor Object Reference") (`Target Location` :type "Vector Structure"))
  (`self.CastAbility` `Target Actor` `Target Location` (`self.TapAbility`)))

(event `Cast Hold Ability`
  (params (`Target Actor` :type "Actor Object Reference") (`Target Location` :type "Vector Structure"))
  (`self.CastAbility` `Target Actor` `Target Location` (`self.HoldAbility`)))

(event `Knockup Hold Follow`
  (params (`Target Actor` :type "Actor Object Reference") (`Target Location` :type "Vector Structure") (WhoSetUp :type "/Game/RebuildBPs/Enumerations/CrewEnum Enum" :default "NewEnumerator0"))
  ;[1 1 1] Knockup Hold Follow Ups
  (switch `/Game/RebuildBPs/Enumerations/CrewEnum` WhoSetUp
    (:`NewEnumerator0`
      (`self.CastAbility` `Target Actor` `Target Location` (`self.KnockupHoldFollowCap`)))
    (:`NewEnumerator1`
      (`self.CastAbility` `Target Actor` `Target Location` (`self.KnockupHoldFollowBull`)))
    (:`NewEnumerator2`
      (`self.CastAbility` `Target Actor` `Target Location` (`self.KnockupHoldFollowFire`)))
    (:`NewEnumerator5`
      (`self.CastAbility` `Target Actor` `Target Location` (`self.KnockupHoldFollowWitch`)))))

(event `Knockup Tap Follow`
  (params (`Target Actor` :type "Actor Object Reference") (`Target Location` :type "Vector Structure") (WhoSetUp :type "/Game/RebuildBPs/Enumerations/CrewEnum Enum" :default "NewEnumerator0"))
  ;[1 1 1] Knockup Tap Follow Ups
  (switch `/Game/RebuildBPs/Enumerations/CrewEnum` WhoSetUp
    (:`NewEnumerator0`
      (`self.CastAbility` `Target Actor` `Target Location` (`self.KnockupTapFollowCap`)))
    (:`NewEnumerator1`
      (`self.CastAbility` `Target Actor` `Target Location` (`self.KnockupTapFollowBull`)))
    (:`NewEnumerator2`
      (`self.CastAbility` `Target Actor` `Target Location` (`self.KnockupTapFollowFire`)))
    (:`NewEnumerator5`
      (`self.CastAbility` `Target Actor` `Target Location` (`self.KnockupTapFollowWitch`)))))

(event `AOE Tap Follow`
  (params (`Target Actor` :type "Actor Object Reference") (`Target Location` :type "Vector Structure") (WhoSetUp :type "/Game/RebuildBPs/Enumerations/CrewEnum Enum" :default "NewEnumerator0"))
  ;[1 1 1] AOE Tap Follow Ups
  (switch `/Game/RebuildBPs/Enumerations/CrewEnum` WhoSetUp
    (:`NewEnumerator0`
      (`self.CastAbility` `Target Actor` `Target Location` (`self.AOETapFollowCap`)))
    (:`NewEnumerator1`
      (`self.CastAbility` `Target Actor` `Target Location` (`self.AOETapFollowBull`)))
    (:`NewEnumerator2`
      (`self.CastAbility` `Target Actor` `Target Location` (`self.AOETapFollowFire`)))
    (:`NewEnumerator5`
      (`self.CastAbility` `Target Actor` `Target Location` (`self.AOETapFollowWitch`)))))

(event `AOE Hold Follow`
  (params (`Target Actor` :type "Actor Object Reference") (`Target Location` :type "Vector Structure") (WhoSetUp :type "/Game/RebuildBPs/Enumerations/CrewEnum Enum" :default "NewEnumerator0"))
  ;[1 1 1] AOE Hold Follow Ups
  (switch `/Game/RebuildBPs/Enumerations/CrewEnum` WhoSetUp
    (:`NewEnumerator0`
      (`self.CastAbility` `Target Actor` `Target Location` (`self.AOEHoldFollowCap`)))
    (:`NewEnumerator1`
      (`self.CastAbility` `Target Actor` `Target Location` (`self.AOEHoldFollowBull`)))
    (:`NewEnumerator2`
      (`self.CastAbility` `Target Actor` `Target Location` (`self.AOEHoldFollowFire`)))
    (:`NewEnumerator5`
      (`self.CastAbility` `Target Actor` `Target Location` (`self.AOEHoldFollowWitch`)))))

(fn `UserConstructionScript`
  (`parent.UserConstructionScript`))