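; BullAntRBP is the bull ant crewmember Blueprint, adding a charge that temporarily boosts its movement.
; StartCharge sharply raises the CharacterMovement max acceleration and walk speed, and EndCharge sets both back to fixed normal values.
; The AbilityEnded override calls EndCharge before passing to the parent, so the boost is cleared when the ability finishes.
; Nothing in this file calls StartCharge, and all other active logic defers to the parent class.
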(event `self.ReceiveBeginPlay`
  (`parent.ReceiveBeginPlay`))

(event `StartCharge`
  (bind _charactermovement (`self.CharacterMovement`))
  (set `CharacterMovementComponent.MaxAcceleration` 8000.0 _charactermovement)
  (set `CharacterMovementComponent.MaxWalkSpeed` 8000.0 _charactermovement))

(event `EndCharge`
  (bind _charactermovement (`self.CharacterMovement`))
  (set `CharacterMovementComponent.MaxAcceleration` 2048.0 _charactermovement)
  (set `CharacterMovementComponent.MaxWalkSpeed` 600.0 _charactermovement))

(event `/Game/RebuildBPs/BaseCharacterRBP.AbilityEnded`
  (`self.EndCharge`)
  (`parent.AbilityEnded`))

(fn `UserConstructionScript`
  (`parent.UserConstructionScript`))