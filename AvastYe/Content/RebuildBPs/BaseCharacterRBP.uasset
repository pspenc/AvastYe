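; Base character Blueprint for team-tagged combatants, handling melee, ranged, abilities, sprint, dash and block.
; BeginPlay optionally loads health and movement stats from a DataTable cached in the GameInstance, then links child-actor weapons.
; Attack montages chain through windup, swing and winddown events that drive weapon traces and trails.
; Incoming hits pass blocking, resistance and team checks before applying damage, knockback, timed hitstun, death or attached status-effect actors.
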(event `self.ReceiveBeginPlay`
  (bind _result (message `/Game/RebuildBPs/Interfaces/GameInstanceInterface.UseCharacterDataTable` (`GameplayStatics.GetGameInstance`)))
  (if (and _result (not (`self.IgnoreANYStatOverrides`)))
    (`self.DrawFromDataTable`))
  (`|ExecutionSequence`
    (:`then_0`
      (set `self.MaxHealth` (`self.Health`)))
    (:`then_1`
      (if (`BlueprintGameplayTagLibrary.HasTag` (`self.GameplayTags`) (struct :`TagName` "Team.GoodGuy"))
        (set `self.Enemy Team` (struct :`TagName` "Team.BadGuy"))
        (else
          (set `self.Enemy Team` (struct :`TagName` "Team.GoodGuy")))))
    (:`then_2`
      (bind _asbase_melee_weapon_rbp (cast `/Game/RebuildBPs/Weapons/BaseMeleeWeaponRBP` (`ChildActorComponent.ChildActor` (`self.MeleeWeapon`))))
      (bind _output_get (set `self.MeleeWeaponReference` _asbase_melee_weapon_rbp))
      (`/Game/RebuildBPs/Weapons/BaseWeaponRBP.AttachOwner` _output_get self))
    (:`then_3`
      (bind _asbase_ranged_weapon_rbp (cast `/Game/RebuildBPs/Weapons/BaseRangedWeaponRBP` (`ChildActorComponent.ChildActor` (`self.RangedWeapon`))))
      (bind _output_get_2 (set `self.RangedWeaponReference` _asbase_ranged_weapon_rbp))
      (`/Game/RebuildBPs/Weapons/BaseWeaponRBP.AttachOwner` _output_get_2 self))
    (:`then_4`
      (set `CharacterMovementComponent.MaxWalkSpeed` (`self.NormalSpeed`) (`self.CharacterMovement`)))))

(event `Sprint`
  (bind _charactermovement (`self.CharacterMovement`))
  (set `CharacterMovementComponent.MaxWalkSpeed` (`self.SprintSpeed`) _charactermovement)
  (set `CharacterMovementComponent.MaxAcceleration` (`self.SprintAcceleration`) _charactermovement))

(event `StopSprint`
  (bind _charactermovement (`self.CharacterMovement`))
  (set `CharacterMovementComponent.MaxWalkSpeed` (`self.NormalSpeed`) _charactermovement)
  (set `CharacterMovementComponent.MaxAcceleration` (`self.NormalAcceleration`) _charactermovement))

(event `/Game/RebuildBPs/Interfaces/DamageInterface.GetDamaged`
  (params (Damage :type "Float (single-precision)") (Hitstun :type "Float (single-precision)") (ForceVector :type "Vector Structure") (`Damage Type` :type "/Game/RebuildBPs/Enumerations/DamageType Enum" :default "NewEnumerator0") (`Attack Type` :type "/Game/RebuildBPs/Enumerations/AttackType Enum" :default "NewEnumerator0") (Attacker :type "/Game/RebuildBPs/BaseCharacterRBP Object Reference") (`Hit Component` :type "PrimitiveComponent Object Reference") (`Enemy Team` :type "GameplayTag Structure") (`Status Effect` :type "/Game/RebuildBPs/StatusEffects/BaseStatusEffect Class Reference"))
  (bind _blocked (`self.BlockingLogic` Damage `Damage Type` `Attack Type` Attacker `Enemy Team`))
  (if _blocked
    (`self.PostBlock` Attacker)
    (else
      (bind (_new_damage _new_hitstun _new_forcevector _entirely_negated) (`self.ProcessDamageModifications` Damage Hitstun ForceVector `Damage Type` `Attack Type` `Enemy Team`)) ; Modifies damage, and checks for the team
      (if (not _entirely_negated)
        (bind _died (`self.ApplyDamage` _new_damage _new_hitstun _new_forcevector `Damage Type` `Attack Type` Attacker `Hit Component` `Enemy Team`))
        (`self.HitReaction` _new_hitstun)
        (if _died
          (`self.Die`)
          (else
            (`self.ApplyStatusEffects` `Attack Type` `Status Effect` Attacker)))))))

(event `PrepSwing`
  (`self.PlayAnimMontage` (`self.RaiseSwordAnim`)))

(event `Die`
  ;[1 1 1] Die
  (`self.K2_DestroyActor`))

(event `WindupStart`
  (set `self.AttackWindup` true)
  (`self.WhichAttackToCycle`
    (:`Basic`
      (`self.BasicAttackCycling`))
    (:`Heavy`
      (`self.HeavyAttackCycling`))
    (:`Special`)))

(event `SwingStart`
  (set `self.AttackWindup` false)
  (set `self.Attacking` true)
  (`self.BeginWeaponTrail`)
  (`/Game/RebuildBPs/Weapons/BaseMeleeWeaponRBP.InitialAttackTrace` (`self.MeleeWeaponReference`)))

(event `BasicMeleeAttack`
  (if (and (`self.AbleToAttack`) (`self.AbleToAct`) (not (`self.Attacking`)) (not (`self.AttackWindup`)))
    (`self.BasicAttackSwing`)))

(event `SwingEnd`
  (set `self.Attacking` false)
  (`self.EndWeaponTrail`)
  (`/Game/RebuildBPs/Weapons/BaseMeleeWeaponRBP.ClearHitActorsArray` (`self.MeleeWeaponReference`))
  (set `self.AttackWinddown` true)
  (set `self.HeavyAttacking` false)
  (set `self.SpecialAttacking` false))

(event `GetHealed`
  (params (`Heal Amount` :type "Float (double-precision)"))
  (set `self.Health` (`KismetMathLibrary.FClamp` (+ (`self.Health`) `Heal Amount`) 0.0 (`self.MaxHealth`))))

(event `WindDownEnd`
  (set `self.AttackWinddown` false)
  (`KismetSystemLibrary.Delay` 0.2)
  (set `self.BasicAttackChainIndex` 0)
  (set `self.HeavyAttackChainIndex` 0))

(event `HeavyAttack`
  (if (and (`self.AbleToAttack`) (`self.AbleToAct`) (not (`self.Attacking`)) (not (`self.AttackWindup`)))
    (`self.HeavyAttackSwing`)))

(event `HitReaction`
  (params (Hitstun :type "Float (double-precision)"))
  (if (> Hitstun 0.0)
    (`self.InteruptAttackLogic`)
    (`self.PlayAnimMontage` (`self.HitAnimation`) :!label _label)
    (elif (not (or (`self.Attacking`) (`self.AttackWindup`) (`self.AttackWinddown`)))
      (goto _label))))

(event `PerfectWindowStartNotify`)

(event `Special Attack`
  (if (and (`self.AbleToAttack`) (`self.AbleToAct`) (not (`self.Attacking`)) (not (`self.AttackWindup`)))
    (`self.SpecialAttackSwing`)))

(event `PerfectWindownStopNotify`)

(event `HeavyAttackSwing`
  (set `self.HeavyAttacking` true)
  (`self.PlayAnimMontage` (`|GetArrayItem` (`self.HeavyMeleeAttackMontages`) (`self.HeavyAttackChainIndex`)) (/ (`self.BaseAnimPlayrate`) (`/Game/RebuildBPs/Weapons/BaseMeleeWeaponRBP.Attack Speed` (`self.MeleeWeaponReference`)))))

(event `BasicAttackSwing`
  (`self.PlayAnimMontage` (`|GetArrayItem` (`self.BasicMeleeAttackMontages`) (`self.BasicAttackChainIndex`)) (/ (`self.BaseAnimPlayrate`) (`/Game/RebuildBPs/Weapons/BaseMeleeWeaponRBP.Attack Speed` (`self.MeleeWeaponReference`)))))

(event `StartPerfectWindow`
  (params (AttackingActor :type "/Game/RebuildBPs/BaseCharacterRBP Object Reference")))

(event `EndPerfectWindow`)

(event `SpecialAttackSwing`
  (set `self.SpecialAttacking` true)
  (`self.PlayAnimMontage` (`self.SpecialAttackMontage`) (/ (`self.BaseAnimPlayrate`) (`/Game/RebuildBPs/Weapons/BaseMeleeWeaponRBP.Attack Speed` (`self.MeleeWeaponReference`)))))

(event `InteruptAttackLogic`
  (bind _meleeweaponreference (`self.MeleeWeaponReference`))
  (set `self.Attacking` false)
  (`self.EndWeaponTrail`)
  (`/Engine/EditorBlueprintResources/StandardMacros.IsValid` _meleeweaponreference
    (:`Is Valid`
      (`/Game/RebuildBPs/Weapons/BaseMeleeWeaponRBP.ClearHitActorsArray` _meleeweaponreference)
      (set `self.HeavyAttacking` false)
      (set `self.SpecialAttacking` false)
      (set `self.AttackWindup` false)
      (set `self.AttackWinddown` false)
      (set `self.BasicAttackChainIndex` 0)
      (set `self.HeavyAttackChainIndex` 0))))

(event `RangedAttack`
  (params (`Target Actor` :type "Actor Object Reference") (`Target Location` :type "Vector Structure"))
  ;[1 1 1] Ranged Attack
  (`/Game/RebuildBPs/Weapons/BaseRangedWeaponRBP.Shoot` (`self.RangedWeaponReference`) `Target Actor` `Target Location`))

(event `BeginWeaponTrail`
  (bind _meleeweaponreference (`self.MeleeWeaponReference`))
  (`/Engine/EditorBlueprintResources/StandardMacros.IsValid` _meleeweaponreference
    (:`Is Valid`
      (`/Game/RebuildBPs/Weapons/BaseMeleeWeaponRBP.Start Sword Trail` _meleeweaponreference))))

(event `AbilityEnded`)

(event `EndWeaponTrail`
  (bind _meleeweaponreference (`self.MeleeWeaponReference`))
  (`/Engine/EditorBlueprintResources/StandardMacros.IsValid` _meleeweaponreference
    (:`Is Valid`
      (`/Game/RebuildBPs/Weapons/BaseMeleeWeaponRBP.End Sword Trail` _meleeweaponreference))))

(event `Dash`
  (params (`Dash Direction` :type "Vector Structure") (`Dash Forward` :type "Float (double-precision)") (`Dash Up` :type "Float (double-precision)"))
  (bind _charactermovement (`self.CharacterMovement`))
  ;[1 1 1] Dash
  (`self.CanDashMacro`
    (:`Can Dash`
      (`self.InteruptAttackLogic`)
      (`self.PlayAnimMontage` (`self.DashAnimation`))
      (set `self.IsDashing` true)
      (set `CharacterMovementComponent.GroundFriction` 0.0 (`self.CharacterMovement`))
      (set `self.AbleToMove` false)
      (`self.LaunchCharacter` (`/Game/RebuildBPs/FunctionMacroLibraries/AvastYeActorMacros.Make Force Vector` `Dash Direction` `Dash Forward` `Dash Up`) true true)
      (`KismetSystemLibrary.Delay` 0.5)
      (set `self.IsDashing` false)
      (`self.DashEnded`)
      (set `CharacterMovementComponent.GroundFriction` 8.0 _charactermovement)
      (`MovementComponent.StopMovementImmediately` _charactermovement)
      (set `self.AbleToMove` true))))

(event `DashEnded`
  ;[1 1 1] Dash
)

(event `GetMoved`
  (params (MoveFromLocation :type "Vector Structure") (MoveToLocation :type "Vector Structure") (PlayRate :type "Float (double-precision)" :default 1.0) (Arc :type "Float (double-precision)"))
  ;[1 1 1] get Moved
  (`TimelineComponent.SetPlayRate` (`self.GetMovedTimline`) PlayRate)
  (bind (_direction _newtrack_0 _z) (`Timeline|GetMovedTimline` :!via `PlayFromStart`)
    (:`Update`
      (bind (_returnvalue_x _returnvalue_y _returnvalue_z) (`KismetMathLibrary.BreakVector` (`KismetMathLibrary.VLerp` MoveFromLocation MoveToLocation _newtrack_0)))
      (`self.K2_SetActorLocation` (`KismetMathLibrary.MakeVector` _returnvalue_x _returnvalue_y (+ (`KismetMathLibrary.Lerp` 0.0 Arc _z) _returnvalue_z))))))

(event `Block`
  (`self.CanBlockMacro`
    (:`Can Block`
      (set `self.IsBlocking` true)
      (set `self.AbleToMove` false)
      (`self.InteruptAttackLogic`)
      (bind _returnvalue (`self.PlayAnimMontage` (`self.BlockAnimation`)))
      (`KismetSystemLibrary.Delay` _returnvalue)
      (`self.EndBlock`))))

(event `EndBlock`
  (set `self.IsBlocking` false)
  (set `self.AbleToMove` true))

(fn `ApplyDamage`
  (params (Damage :type "Float (double-precision)") (Hitstun :type "Float (double-precision)") (ForceVector :type "Vector Structure") (`Damage Type` :type "/Game/RebuildBPs/Enumerations/DamageType Enum" :default "NewEnumerator0") (`Attack Type` :type "/Game/RebuildBPs/Enumerations/AttackType Enum" :default "NewEnumerator0") (Attacker :type "/Game/RebuildBPs/BaseCharacterRBP Object Reference") (`Hit Component` :type "PrimitiveComponent Object Reference") (`Team to Damage` :type "GameplayTag Structure"))
  (returns (Died :type Boolean))
  (if (`GameplayTagAssetInterface.HasMatchingGameplayTag` self `Team to Damage`)
    (for _array_element (`self.StatusEffectList`)
      (`/Game/RebuildBPs/StatusEffects/BaseStatusEffect.Owner Damaged` _array_element `Damage Type` `Attack Type`))
    (bind _output_get (set `self.Health` (- (`self.Health`) Damage)))
    (bind _returnvalue (<= _output_get 0.0))
    (if _returnvalue
      (return _returnvalue)
      (else
        (`self.LaunchCharacter` ForceVector true true)
        (`self.ApplyHitstun` Hitstun)
        (return false)))))

(fn `ApplyHitstun`
  (params (Hitstun :type "Float (double-precision)"))
  (if (> Hitstun 0.0)
    (set `self.AbleToAct` false)
    (if (>= Hitstun (`KismetSystemLibrary.K2_GetTimerRemainingTimeHandle` (`self.HitstunTimerHandle`)))
      (bind _returnvalue (`KismetSystemLibrary.K2_SetTimer` self "ClearStunned" Hitstun))
      (set `self.HitstunTimerHandle` _returnvalue))))

(fn `ApplyStatusEffects`
  (params (`Attack Type` :type "/Game/RebuildBPs/Enumerations/AttackType Enum" :default "NewEnumerator0") (`Status Effect` :type "/Game/RebuildBPs/StatusEffects/BaseStatusEffect Class Reference") (Attacker :type "/Game/RebuildBPs/BaseCharacterRBP Object Reference"))
  (returns (`Effect Applied` :type Boolean))
  (locals (`Dont Apply` :type Boolean))
  (if (or (== `Status Effect` "/Game/RebuildBPs/StatusEffects/BaseStatusEffect.BaseStatusEffect_C") (== `Status Effect` null))
    (return false)
    (else
      (for _array_element (`self.StatusEffectList`)
        (bind _returnvalue (`GameplayStatics.GetObjectClass` _array_element))
        (if (== `Status Effect` _returnvalue)
          (if (defaults `/Game/RebuildBPs/BaseCharacterRBP` _returnvalue)
            (`/Game/RebuildBPs/StatusEffects/BaseStatusEffect.FinishStatusEffect` _array_element)
            (break)
            (else
              (set `local.Dont Apply` true)
              (break)))))
      (if (not (`local.Dont Apply`))
        (bind _returnvalue_2 (`|SpawnActorFromClass` `Status Effect` (`KismetMathLibrary.MakeTransform` (`self.K2_GetActorLocation`)) "AlwaysSpawn" "OverrideRootScale" self self Attacker null))
        (`self.K2_AttachToActor` _returnvalue_2 self "None" "SnapToTarget" "SnapToTarget" "KeepRelative" true)
        (`/Game/RebuildBPs/StatusEffects/BaseStatusEffect.OnAttach` _returnvalue_2)
        (`KismetArrayLibrary.Array_Add` (`self.StatusEffectList`) _returnvalue_2)
        (`KismetArrayLibrary.Array_AddUnique` (`self.StatusEffectClassList`) (`GameplayStatics.GetObjectClass` _returnvalue_2))
        (return true)))))

(fn `BasicAttackCycling`
  (bind _result (`/Engine/EditorBlueprintResources/StandardMacros.IncrementInt` (`self.BasicAttackChainIndex`))
    (:`  `
      (if (>= _result (`KismetArrayLibrary.Array_Length` (`self.BasicMeleeAttackMontages`)))
        (set `self.BasicAttackChainIndex` 0))
      (return))))

(fn `BlockingLogic`
  (params (Damage :type "Float (double-precision)") (`Damage Type` :type "/Game/RebuildBPs/Enumerations/DamageType Enum" :default "NewEnumerator0") (`Attack Type` :type "/Game/RebuildBPs/Enumerations/AttackType Enum" :default "NewEnumerator0") (Attacker :type "/Game/RebuildBPs/BaseCharacterRBP Object Reference") (`Enemy Team` :type "GameplayTag Structure"))
  (returns (Blocked :type Boolean))
  (return (and (`|EnumInequality` `Damage Type` "NewEnumerator2") (`self.IsBlocking`))))

(fn `CastAbility`
  (params (TargetActor :type "Actor Object Reference") (TargetLocation :type "Vector Structure") (Ability :type "/Game/RebuildBPs/Abilities/BaseAbility Class Reference"))
  (returns (AbilityObject :type "/Game/RebuildBPs/Abilities/BaseAbility Object Reference"))
  (bind _returnvalue (`|SpawnActorFromClass` Ability (`self.GetTransform`) "AlwaysSpawn" "OverrideRootScale" self self TargetActor TargetLocation null))
  (`/Game/RebuildBPs/Abilities/BaseAbility.StartAbility` _returnvalue)
  (return _returnvalue))

(fn `ClearStunned`
  (set `self.AbleToAct` true))

(fn `DrawFromDataTable`
  (bind _characterdisplayname (`self.CharacterDisplayName`))
  (bind (_data _data_found) (message `/Game/RebuildBPs/Interfaces/GameInstanceInterface.GetPreLoadedCharacterData` (`GameplayStatics.GetGameInstance`) (`self.CharacterDisplayName`)))
  (if _data_found
    (`KismetSystemLibrary.PrintString` (`KismetStringLibrary.Concat_StrStr` (`KismetStringLibrary.Conv_NameToString` (`self.CharacterDisplayName`)) "  Already Loaded") false)
    (bind (_health _normalspeed _normalacceleration _sprintspeed _sprintacceleration) (break `/Game/RebuildBPs/CharacterStatContainers/CharacterStatsStruct` (`.BasicStats_26_9C1BBFDD497605C8DB216F90EF2800C5` (break `/Game/RebuildBPs/Structs/NewCharacterStruct` _data))))
    (set `self.Health` _health)
    (set `self.NormalSpeed` _normalspeed)
    (set `self.NormalAcceleration` _normalacceleration)
    (set `self.SprintSpeed` _sprintspeed)
    (set `self.SprintAcceleration` _sprintacceleration)
    (else
      (bind _returnvalue (`|GetDataTableRow` "/Game/RebuildBPs/CharacterDataTable.CharacterDataTable" _characterdisplayname)
        (:`then`
          (`KismetSystemLibrary.PrintString` (`KismetStringLibrary.Concat_StrStr` (`KismetStringLibrary.Conv_NameToString` _characterdisplayname) "  DATA FOUND") false)
          (bind (_health_2 _normalspeed_2 _normalacceleration_2 _sprintspeed_2 _sprintacceleration_2) (break `/Game/RebuildBPs/CharacterStatContainers/CharacterStatsStruct` (`.BasicStats_26_9C1BBFDD497605C8DB216F90EF2800C5` (break `/Game/RebuildBPs/Structs/NewCharacterStruct` _returnvalue))))
          (set `self.Health` _health_2)
          (set `self.NormalSpeed` _normalspeed_2)
          (set `self.NormalAcceleration` _normalacceleration_2)
          (set `self.SprintSpeed` _sprintspeed_2)
          (set `self.SprintAcceleration` _sprintacceleration_2)
          (message `/Game/RebuildBPs/Interfaces/GameInstanceInterface.StoreLoadedCharacter` (`GameplayStatics.GetGameInstance`) (`self.CharacterDisplayName`) _returnvalue))
        (:`RowNotFound`
          (if (== _characterdisplayname "Null")
            (`KismetSystemLibrary.PrintString` (`KismetStringLibrary.Concat_StrStr` (`KismetStringLibrary.Conv_NameToString` _characterdisplayname) " DATA NOT FOUND") false)))))))

(fn `HasStatusEffect`
  (params (`Effect to Check` :type "/Game/RebuildBPs/StatusEffects/BaseStatusEffect Class Reference"))
  (returns (`Has Effect` :type Boolean))
  (return (!= (`KismetArrayLibrary.Array_Find` (`self.StatusEffectClassList`) `Effect to Check`) -1)))

(fn `HeavyAttackCycling`
  (bind _result (`/Engine/EditorBlueprintResources/StandardMacros.IncrementInt` (`self.HeavyAttackChainIndex`))
    (:`  `
      (if (>= _result (`KismetArrayLibrary.Array_Length` (`self.HeavyMeleeAttackMontages`)))
        (set `self.HeavyAttackChainIndex` 0))
      (return))))

(fn `PostBlock`
  (params (`Blocked Attacker` :type "/Game/RebuildBPs/BaseCharacterRBP Object Reference"))
  (set `self.IsBlocking` false))

(fn `ProcessDamageModifications`
  (params (`Base Damage` :type "Float (double-precision)") (`Base Hitstun` :type "Float (double-precision)") (ForceVector :type "Vector Structure") (`Damage Type` :type "/Game/RebuildBPs/Enumerations/DamageType Enum" :default "NewEnumerator0") (`Attack Type` :type "/Game/RebuildBPs/Enumerations/AttackType Enum" :default "NewEnumerator0") (TeamToDamage :type "GameplayTag Structure"))
  (returns (`New Damage` :type "Float (double-precision)") (`New Hitstun` :type "Float (double-precision)") (`New ForceVector` :type "Vector Structure") (`Entirely Negated` :type Boolean))
  (bind _returnvalue (* (`BlueprintMapLibrary.Map_Find` (`self.DamageResistances`) `Damage Type`) `Base Damage`))
  (if (`GameplayTagAssetInterface.HasMatchingGameplayTag` self TeamToDamage)
    (return _returnvalue `Base Hitstun` ForceVector (and (<= _returnvalue 0.0) (!= `Base Damage` 0.0)))
    (else
      (return _returnvalue `Base Hitstun` ForceVector true))))

(fn `UserConstructionScript`)