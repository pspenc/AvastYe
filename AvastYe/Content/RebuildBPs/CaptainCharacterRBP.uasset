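; Player captain character that handles movement, melee, dash and abilities, and commands a crew (BullAnt, FireAnt, WitchDoctor) through a CaptainingComponent.
; Crew buttons use timers to separate tap from hold, switching to follow-up commands during knockup or magic/fire quick-time windows, which open with brief slow motion and blur.
; Combat entry and exit notify crew AI and toggle timed directional auto-lock targeting, while abilities aim via widening camera-forward sphere traces.
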(event `InputAction|SlashAttack`
  (params (Key :type "Key Structure"))
  ;[1 1 1] INPUTS
  (:`Pressed`
    (`self.BasicMeleeAttack`)))

(event `InputAction|BullAnt`
  (params (Key :type "Key Structure"))
  ;[1 1 1] INPUTS
  ;;[1 1 1] Crew Inputs
  (:`Pressed`
    (`self.BullAntPressed`))
  (:`Released`
    (`self.BullAntReleased`)))

(event `InputAction|StabAttack`
  (params (Key :type "Key Structure"))
  ;[1 1 1] INPUTS
)

(event `InputAction|OptionsMenu`
  (params (Key :type "Key Structure"))
  ;[1 1 1] INPUTS
)

(event `InputAction|FireAnt`
  (params (Key :type "Key Structure"))
  ;[1 1 1] INPUTS
  ;;[1 1 1] Crew Inputs
  (:`Pressed`
    (`self.FireAntPressed`))
  (:`Released`
    (`self.FireAntReleased`)))

(event `InputAxis|MoveForward` :overrideparent false
  (params (AxisValue :type "Float (single-precision)"))
  ;[1 1 1] Movement and Camera Input
  (if (and (`self.AbleToMove`) (`self.AbleToAct`))
    (`self.AddMovementInput` (`KismetMathLibrary.GetForwardVector` (`KismetMathLibrary.MakeRotator` 0.0 0.0 (.yaw (`self.GetControlRotation`)))) AxisValue)))

(event `InputAction|Grapple/CaptainFollow`
  (params (Key :type "Key Structure"))
  ;[1 1 1] INPUTS
)

(event `InputAction|WitchDoctor`
  (params (Key :type "Key Structure"))
  ;[1 1 1] INPUTS
  ;;[1 1 1] Crew Inputs
  (:`Pressed`
    (`self.WitchDoctorPressed`))
  (:`Released`
    (`self.WitchDoctorReleased`)))

(event `InputAction|Dash`
  (params (Key :type "Key Structure"))
  ;[1 1 1] INPUTS
)

(event `InputAction|Block`
  (params (Key :type "Key Structure"))
  ;[1 1 1] INPUTS
)

(event `InputAxis|MoveRight` :overrideparent false
  (params (AxisValue :type "Float (single-precision)"))
  ;[1 1 1] Movement and Camera Input
  (if (and (`self.AbleToMove`) (`self.AbleToAct`))
    (`self.AddMovementInput` (`KismetMathLibrary.GetRightVector` (`KismetMathLibrary.MakeRotator` 0.0 0.0 (.yaw (`self.GetControlRotation`)))) AxisValue)))

(event `InputAction|Sprint`
  (params (Key :type "Key Structure"))
  ;[1 1 1] INPUTS
)

(event `InputAxis|Turn` :overrideparent false
  (params (AxisValue :type "Float (single-precision)"))
  ;[1 1 1] Movement and Camera Input
  (`self.AddControllerYawInput` AxisValue))

(event `Enter Combat`
  ;[1 1 1] Enter/Exit Combat
  (`KismetSystemLibrary.Delay` 0.2)
  (if (not (`self.InCombat`))
    (set `self.InCombat` true)
    (for _array_element (`self.The Crew`)
      (message `/Game/BPs/Interfaces/AICommunicationInterface.CrewEnterCombat` (`AIBlueprintHelperLibrary.GetAIController` _array_element))
      (bind _returnvalue (`KismetSystemLibrary.K2_SetTimer` null "AutoLockTargeting" 0.1 true)))))

(event `InputAxis|LookUp` :overrideparent false
  (params (AxisValue :type "Float (single-precision)"))
  ;[1 1 1] Movement and Camera Input
  (`self.AddControllerPitchInput` AxisValue))

(event `ExitCombat`
  ;[1 1 1] Enter/Exit Combat
  (`KismetSystemLibrary.Delay` 0.5)
  (bind _outactors (`GameplayStatics.GetAllActorsOfClass` "/Game/RebuildBPs/AI/EnemyAIDirectorR.EnemyAIDirectorR_C"))
  (`/Game/BPs/MacroFunctionLibraries/MoreporkMacros.Array Length Int Compare` _outactors
    (:`>`
      (for _array_element _outactors
        (if (`/Game/RebuildBPs/AI/EnemyAIDirectorR.IsActivated` _array_element)
          (set `self.There is another active director` true)
          (break)
          (else
            (set `self.There is another active director` false))))
      (if (not (`self.There is another active director`))
        (set `self.InCombat` false :!label _label)
        (set `self.Health` (`self.MaxHealth`))
        (`/Game/BPs/CaptainingComponent.Exit Combat` (`self.CaptainingComponent`))
        (`/Game/BPs/Camera/PlayerCameraManager.End Combat` (`self.PlayerCameraManager`))
        (for _array_element_2 (`self.The Crew`)
          (message `/Game/BPs/Interfaces/AICommunicationInterface.CrewLeaveCombat` (`AIBlueprintHelperLibrary.GetAIController` _array_element_2)))
        (`KismetSystemLibrary.K2_ClearAndInvalidateTimerHandle` (stale `Enter Combat` _returnvalue))))
    (:`==`
      (goto _label))
    (:`<`
      (goto _label))))

(event `Key|LeftMouseButton`
  (params (Key :type "Key Structure"))
  ;[0 1 0.9558] PATRICK'S TESTING STUFF
  (:`Pressed`
    (`self.BasicMeleeAttack`)))

(event `SetTarget`
  (params (NewTarget :type "/Game/RebuildBPs/AI/BaseEnemyAIRBP Object Reference"))
  (bind _combattarget (`self.CombatTarget`))
  ;[1 1 1] Set Combat Target
  (if (not (== NewTarget _combattarget))
    (`/Engine/EditorBlueprintResources/StandardMacros.IsValid` _combattarget
      (:`Is Valid`
        (`/Game/RebuildBPs/AI/BaseEnemyAIRBP.Get UnTargeted` _combattarget))
      (:`Is Not Valid`
        _))
    (bind _output_get (set `self.CombatTarget` NewTarget))
    (`/Engine/EditorBlueprintResources/StandardMacros.IsValid` _output_get
      (:`Is Valid`
        (`/Game/RebuildBPs/AI/BaseEnemyAIRBP.Get Targeted` _output_get)))))

(event `Key|MiddleMouseButton`
  (params (Key :type "Key Structure"))
  ;[0 1 0.9558] PATRICK'S TESTING STUFF
  (:`Pressed`
    (bind (_target_actor _successful) (`self.Targetting`))
    (if _successful
      (`self.RangedAttack` _target_actor (`self.K2_GetActorLocation` _target_actor)))))

(event `Key|One`
  (params (Key :type "Key Structure"))
  ;[0 1 0.9558] PATRICK'S TESTING STUFF
  (:`Pressed`
    (bind (_target_actor _successful) (`self.Targetting`))
    (if _successful
      (`self.CastAbility` _target_actor (0.0 0.0 0.0) "/Game/RebuildBPs/Abilities/GroundSlamAbility.GroundSlamAbility_C"))))

(event `Key|Three`
  (params (Key :type "Key Structure"))
  ;[0 1 0.9558] PATRICK'S TESTING STUFF
  (:`Pressed`
    (bind (_target_actor _successful) (`self.Targetting`))
    (if _successful
      (`self.CastAbility` _target_actor (0.0 0.0 0.0) "/Game/RebuildBPs/Abilities/BlackHoleAbility.BlackHoleAbility_C"))))

(event `Key|Two`
  (params (Key :type "Key Structure"))
  ;[0 1 0.9558] PATRICK'S TESTING STUFF
  (:`Pressed`
    (`self.CastAbility` null (0.0 0.0 0.0) "/Game/RebuildBPs/Abilities/FlameBreathAbility.FlameBreathAbility_C")))

(event `Key|SpaceBar`
  (params (Key :type "Key Structure"))
  ;[0 1 0.9558] PATRICK'S TESTING STUFF
  (:`Pressed`
    (`self.Dash` (`self.GetLastMovementInputVector`) 2000.0 100.0)))

(event `RFBMaxHold`
  ;[1 1 1] Crew Abilities
  (set `self.RFBHeldMax` true)
  (if (or (`self.KnockupQuickTimeAvailable`) (`self.Magic/FireQuickTimeAvailable`))
    (`self.BullFollowUpHold`)
    (else
      (`/Game/BPs/CaptainingComponent.BullHold` (`self.CaptainingComponent`))
      (message `/Game/BPs/Interfaces/GameModeInterface.CaptainCommandedBullSlam` (`GameplayStatics.GetGameMode`)))))

(event `RFBHeldTimer`
  ;[1 1 1] Crew Abilities
  (`/Engine/EditorBlueprintResources/StandardMacros.IncrementFloat` (`self.RFBHeldDuration`)))

(event `AlertOfQuickTime`
  (params (`Quick Time Type` :type "/Game/BPs/GlobalEnums/QuickTimeEnum Enum" :default "NewEnumerator0") (Target :type "Actor Object Reference") (RequiredFocusBars :type Integer) (CausedByEnv :type Boolean) (WhoSetUp :type "Actor Object Reference"))
  (bind _mainhud (`self.MainHud`))
  (bind _followupduration (`self.FollowUpDuration`))
  ;[1 1 1] Alert Captain of Follow Up
  (if CausedByEnv
    _
    (else
      _))
  (set `self.WhoSetUp` WhoSetUp)
  (switch `/Game/BPs/GlobalEnums/QuickTimeEnum` `Quick Time Type`
    (:`NewEnumerator0`
      (if (not (`self.KnockupQuickTimeAvailable`))
        (set `self.KnockupQuickTimeAvailable` true)
        (bind _output_get (set `self.KnockupQuickTimeTarget` Target))
        (`self.ActivateFollowUpTargetDispatcher` _output_get)
        (`KismetSystemLibrary.K2_SetTimerDelegate` (delegate `ClearKnockupQuickTime`) _followupduration)
        (`/Engine/EditorBlueprintResources/StandardMacros.IsValid` _output_get
          (:`Is Valid`
            (`GameplayStatics.SetGlobalTimeDilation` 0.1 :!label _label_2)
            (`/Game/BPs/UI/MainHUD.StartBlur` _mainhud)
            (`KismetSystemLibrary.Delay` 0.0225)
            (`GameplayStatics.SetGlobalTimeDilation` 1.0)
            (`/Game/BPs/UI/MainHUD.EndBlur` _mainhud)))))
    (:`NewEnumerator1`
      (if (not (`self.Magic/FireQuickTimeAvailable`))
        (set `self.Magic/FireQuickTimeAvailable` true)
        (bind _output_get_2 (set `self.Magic/FireQuickTimeTarget` Target))
        (`self.ActivateFollowUpTargetDispatcher` _output_get_2)
        (`KismetSystemLibrary.K2_SetTimerDelegate` (delegate `ClearMagic/FireQuickTime`) _followupduration)
        (`/Engine/EditorBlueprintResources/StandardMacros.IsValid` _output_get_2
          (:`Is Valid`
            (goto _label_2)))))))

(event `BullAntPressed`
  ;[1 1 1] Crew Abilities
  (`/Engine/EditorBlueprintResources/StandardMacros.DoOnce` false :!label _label_3
    (:`Completed`
      (bind _returnvalue (`KismetSystemLibrary.K2_SetTimerDelegate` (delegate `RFBHeldTimer`) 0.1 true))
      (bind _returnvalue_2 (`KismetSystemLibrary.K2_SetTimerDelegate` (delegate `RFBMaxHold`) 0.5)))))

(event `ClearKnockupQuickTime`
  ;[1 1 1] Alert Captain of Follow Up
  (set `self.KnockupQuickTimeAvailable` false)
  (`self.ClearFollowUpTargetDispatcher` (`self.KnockupQuickTimeTarget`))
  (set `self.KnockupQuickTimeTarget` null)
  (`GameplayStatics.SetGlobalTimeDilation` 1.0)
  (set `self.WhoSetUp` null :!label _label_4)
  (`/Game/BPs/UI/MainHUD.EndBlur` (`self.MainHud`)))

(event `BullAntReleased`
  (bind _returnvalue (`GameplayStatics.GetGameMode`))
  (bind _captainingcomponent (`self.CaptainingComponent`))
  (bind _returnvalue_2 (or (`self.KnockupQuickTimeAvailable`) (`self.Magic/FireQuickTimeAvailable`)))
  ;[1 1 1] Crew Abilities
  (`KismetSystemLibrary.K2_ClearAndInvalidateTimerHandle` (stale `BullAntPressed` _returnvalue))
  (`KismetSystemLibrary.K2_ClearAndInvalidateTimerHandle` (stale `BullAntPressed` _returnvalue_2))
  (if (`self.RFBHeldMax`)
    (set `self.RFBHeldMax` false)
    (elif (>= (`self.RFBHeldDuration`) 3.0)
      (if _returnvalue_2
        (`self.BullFollowUpHold`)
        (else
          (`/Game/BPs/CaptainingComponent.BullHold` _captainingcomponent)
          (message `/Game/BPs/Interfaces/GameModeInterface.CaptainCommandedBullSlam` _returnvalue)))
      (elif _returnvalue_2
        (`self.BullFollowUpTap`)
        (else
          (`/Game/BPs/CaptainingComponent.BullTap` _captainingcomponent)
          (message `/Game/BPs/Interfaces/GameModeInterface.CaptainCommandedBullCharge` _returnvalue)))))
  (set `self.RFBHeldDuration` 0.0)
  (goto _label_3 :!via `Reset`))

(event `ClearMagic/FireQuickTime`
  ;[1 1 1] Alert Captain of Follow Up
  (set `self.Magic/FireQuickTimeAvailable` false)
  (`self.ClearFollowUpTargetDispatcher` (`self.Magic/FireQuickTimeTarget`))
  (set `self.Magic/FireQuickTimeTarget` null)
  (`GameplayStatics.SetGlobalTimeDilation` 1.0)
  (goto _label_4))

(event `TFBMaxHold`
  ;[1 1 1] Crew Abilities
  (set `self.TFBHeldMax` true)
  (if (or (`self.KnockupQuickTimeAvailable`) (`self.Magic/FireQuickTimeAvailable`))
    (`self.WitchDoctorFollowUpHold`)
    (else
      (`/Game/BPs/CaptainingComponent.ThirdHold` (`self.CaptainingComponent`)))))

(event `TFBHeldTimer`
  ;[1 1 1] Crew Abilities
  (`/Engine/EditorBlueprintResources/StandardMacros.IncrementFloat` (`self.TFPHeldDuration`)))

(event `WitchDoctorPressed`
  ;[1 1 1] Crew Abilities
  (`/Engine/EditorBlueprintResources/StandardMacros.DoOnce` false :!label _label_5
    (:`Completed`
      (bind _returnvalue (`KismetSystemLibrary.K2_SetTimerDelegate` (delegate `TFBHeldTimer`) 0.1 true))
      (bind _returnvalue_2 (`KismetSystemLibrary.K2_SetTimerDelegate` (delegate `TFBMaxHold`) 0.5)))))

(event `CaptainFollowUpClicked`
  ;[1 1 1] Follow Ups
  (if (`self.KnockupQuickTimeAvailable`)
    (if (not (== (`self.WhoSetUp`) self))
      (`GameplayStatics.SetGlobalTimeDilation` 1.0))
    (elif (`self.Magic/FireQuickTimeAvailable`)
      (`GameplayStatics.SetGlobalTimeDilation` 1.0)
      (if (== (`self.WhoSetUp`) (`self.FireAnt`))
        _))))

(event `CustomEvent`
  (params (Heavy :type Boolean) (HitActor :type "Actor Object Reference"))
  ;[1 1 1] Focus/Attacks Landing
)

(event `AddFocus`
  (params (FocusGained :type "Float (double-precision)"))
  ;[1 1 1] Focus/Attacks Landing
  (set `self.CurrentFocus` (`KismetMathLibrary.FClamp` (+ (`self.CurrentFocus`) FocusGained) 0.0 (`self.MaxFocus`))))

(event `WitchDoctorReleased`
  (bind _captainingcomponent (`self.CaptainingComponent`))
  (bind _returnvalue (or (`self.KnockupQuickTimeAvailable`) (`self.Magic/FireQuickTimeAvailable`)))
  ;[1 1 1] Crew Abilities
  (`KismetSystemLibrary.K2_ClearAndInvalidateTimerHandle` (stale `WitchDoctorPressed` _returnvalue))
  (`KismetSystemLibrary.K2_ClearAndInvalidateTimerHandle` (stale `WitchDoctorPressed` _returnvalue_2))
  (if (`self.TFBHeldMax`)
    (set `self.TFBHeldMax` false)
    (elif (>= (`self.TFPHeldDuration`) 3.0)
      (if _returnvalue
        (`self.WitchDoctorFollowUpHold`)
        (else
          (`/Game/BPs/CaptainingComponent.ThirdHold` _captainingcomponent)))
      (elif _returnvalue
        (`self.WitchDoctorFollowUpTap`)
        (else
          (`/Game/BPs/CaptainingComponent.ThirdTap` _captainingcomponent)))))
  (set `self.TFPHeldDuration` 0.0)
  (goto _label_5 :!via `Reset`))

(event `UseFocus`
  (params (RequiredFocusBars :type Integer))
  ;[1 1 1] Focus/Attacks Landing
  (set `self.CurrentFocus` (`KismetMathLibrary.FClamp` (- (`self.CurrentFocus`) (* RequiredFocusBars 25.0)) 0.0 (`self.MaxFocus`))))

(event `BullFollowUpTap`
  ;[1 1 1] Follow Ups
  (if (not (== (`self.WhoSetUp`) (`self.BullAnt`)))
    (`GameplayStatics.SetGlobalTimeDilation` 1.0)
    (`/Game/BPs/CaptainingComponent.QuickTimeBullTap` (`self.CaptainingComponent`) (`self.KnockupQuickTimeAvailable`))
    (if (`self.KnockupQuickTimeAvailable`)
      (`self.ClearKnockupQuickTime`)
      (else
        (`self.ClearMagic/FireQuickTime`)))
    (`self.UseFocus` 0)
    (message `/Game/BPs/Interfaces/GameModeInterface.CaptainDidQuickTimeBull` (`GameplayStatics.GetGameMode`))))

(event `BullFollowUpHold`
  ;[1 1 1] Follow Ups
  (if (not (== (`self.WhoSetUp`) (`self.BullAnt`)))
    (`GameplayStatics.SetGlobalTimeDilation` 1.0)
    (`/Game/BPs/CaptainingComponent.QuicktimeBullHold` (`self.CaptainingComponent`) (`self.KnockupQuickTimeAvailable`))
    (if (`self.KnockupQuickTimeAvailable`)
      (`self.ClearKnockupQuickTime`)
      (else
        (`self.ClearMagic/FireQuickTime`)))
    (`self.UseFocus` 0)
    (message `/Game/BPs/Interfaces/GameModeInterface.CaptainDidQuickTimeBull` (`GameplayStatics.GetGameMode`))))

(event `LFBMaxHeld`
  ;[1 1 1] Crew Abilities
  (set `self.LFBHeldMax` true)
  (if (or (`self.KnockupQuickTimeAvailable`) (`self.Magic/FireQuickTimeAvailable`))
    (`self.FireFollowUpHold`)
    (else
      (`/Game/BPs/CaptainingComponent.FireHold` (`self.CaptainingComponent`)))))

(event `LFBHeldTimer`
  ;[1 1 1] Crew Abilities
  (`/Engine/EditorBlueprintResources/StandardMacros.IncrementFloat` (`self.LFBHeldDuration`)))

(event `FireAntPressed`
  ;[1 1 1] Crew Abilities
  (`/Engine/EditorBlueprintResources/StandardMacros.DoOnce` false :!label _label_6
    (:`Completed`
      (bind _returnvalue (`KismetSystemLibrary.K2_SetTimerDelegate` (delegate `LFBHeldTimer`) 0.1 true))
      (bind _returnvalue_2 (`KismetSystemLibrary.K2_SetTimerDelegate` (delegate `LFBMaxHeld`) 0.6)))))

(event `FireFollowUpTap`
  ;[1 1 1] Follow Ups
  (if (not (== (`self.WhoSetUp`) (`self.FireAnt`)))
    (`GameplayStatics.SetGlobalTimeDilation` 1.0)
    (`/Game/BPs/CaptainingComponent.QuickTimeFireTap` (`self.CaptainingComponent`) (`self.KnockupQuickTimeAvailable`))
    (if (`self.KnockupQuickTimeAvailable`)
      (`self.ClearKnockupQuickTime`)
      (else
        (`self.ClearMagic/FireQuickTime`)))
    (`self.UseFocus` 0)
    (message `/Game/BPs/Interfaces/GameModeInterface.CaptainDidQuickTimeFire` (`GameplayStatics.GetGameMode`))))

(event `FireAntReleased`
  (bind _captainingcomponent (`self.CaptainingComponent`))
  (bind _returnvalue (or (`self.KnockupQuickTimeAvailable`) (`self.Magic/FireQuickTimeAvailable`)))
  ;[1 1 1] Crew Abilities
  (`KismetSystemLibrary.K2_ClearAndInvalidateTimerHandle` (stale `FireAntPressed` _returnvalue))
  (`KismetSystemLibrary.K2_ClearAndInvalidateTimerHandle` (stale `FireAntPressed` _returnvalue_2))
  (if (`self.LFBHeldMax`)
    (set `self.LFBHeldMax` false)
    (elif (>= (`self.LFBHeldDuration`) 4.0)
      (if _returnvalue
        (`self.FireFollowUpHold`)
        (else
          (`/Game/BPs/CaptainingComponent.FireHold` _captainingcomponent)))
      (elif _returnvalue
        (`self.FireFollowUpTap`)
        (else
          (`/Game/BPs/CaptainingComponent.FireTap` _captainingcomponent)))))
  (set `self.LFBHeldDuration` 0.0)
  (goto _label_6 :!via `Reset`))

(event `FireFollowUpHold`
  ;[1 1 1] Follow Ups
  (if (not (== (`self.WhoSetUp`) (`self.FireAnt`)))
    (`GameplayStatics.SetGlobalTimeDilation` 1.0)
    (`/Game/BPs/CaptainingComponent.QuickTimeFireHold` (`self.CaptainingComponent`) (`self.KnockupQuickTimeAvailable`))
    (if (`self.KnockupQuickTimeAvailable`)
      (`self.ClearKnockupQuickTime`)
      (else
        (`self.ClearMagic/FireQuickTime`)))
    (`self.UseFocus` 0)
    (message `/Game/BPs/Interfaces/GameModeInterface.CaptainDidQuickTimeFire` (`GameplayStatics.GetGameMode`))))

(event `WitchDoctorFollowUpTap`
  ;[1 1 1] Follow Ups
  (if (not (== (`self.WhoSetUp`) (`self.WitchDoctor`)))
    (`GameplayStatics.SetGlobalTimeDilation` 1.0)
    (`/Game/BPs/CaptainingComponent.QuickTimeWitchTap` (`self.CaptainingComponent`) (`self.KnockupQuickTimeAvailable`))
    (if (`self.KnockupQuickTimeAvailable`)
      (`self.ClearKnockupQuickTime`)
      (else
        (`self.ClearMagic/FireQuickTime`)))
    (`self.UseFocus` 0)
    (message `/Game/BPs/Interfaces/GameModeInterface.CaptainDidQuickTimeWitch` (`GameplayStatics.GetGameMode`))))

(event `WitchDoctorFollowUpHold`
  ;[1 1 1] Follow Ups
  (if (not (== (`self.WhoSetUp`) (`self.WitchDoctor`)))
    (`GameplayStatics.SetGlobalTimeDilation` 1.0)
    (`/Game/BPs/CaptainingComponent.QuickTimeWtichHold` (`self.CaptainingComponent`) (`self.KnockupQuickTimeAvailable`))
    (if (`self.KnockupQuickTimeAvailable`)
      (`self.ClearKnockupQuickTime`)
      (else
        (`self.ClearMagic/FireQuickTime`)))
    (`self.UseFocus` 0)
    (message `/Game/BPs/Interfaces/GameModeInterface.CaptainDidQuickTimeWitch` (`GameplayStatics.GetGameMode`))))

(fn `AutoLockTargeting`
  (locals (TempTargetEnemy :type "/Game/RebuildBPs/AI/BaseEnemyAIRBP Object Reference") (DirectionVector :type "Vector Structure") (PreviousDirectionInput :type "Vector Structure") (Directional :type Boolean) (PriorityAdjustment :type "Float (double-precision)") (TargetingRange :type "Float (double-precision)") (TargetPrority :type "Float (double-precision)"))
  (bind _returnvalue (`self.GetLastMovementInputVector`))
  (bind _temptargetenemy (`local.TempTargetEnemy`))
  ;[1 1 1] if player is not inputting a direction target closest enemy
  (if (== _returnvalue (0.0 0.0 0.0))
    (set `local.DirectionVector` (`self.GetActorForwardVector`))
    (set `local.Directional` false)
    (else
      (set `local.DirectionVector` _returnvalue)
      (set `local.Directional` true)))
  (if (>= (`KismetMathLibrary.DegAcos` (`KismetMathLibrary.Dot_VectorVector` (`KismetMathLibrary.Normal` (`local.PreviousDirectionInput`)) (`KismetMathLibrary.Normal` _returnvalue))) 20.0)
    (bind _outactors (`GameplayStatics.GetAllActorsOfClass` "/Game/RebuildBPs/AI/BaseEnemyAIRBP.BaseEnemyAIRBP_C"))
    (for _array_element _outactors
      (`/Engine/EditorBlueprintResources/StandardMacros.IsValid` _array_element
        (:`Is Valid`
          (if (`local.Directional`)
            (set `local.PriorityAdjustment` 0.0)
            (else
              (bind _returnvalue_2 (- (`self.K2_GetActorLocation` _array_element) (`self.K2_GetActorLocation`)))
              (bind _returnvalue_3 (`KismetMathLibrary.VSize` _returnvalue_2))
              (set `local.PriorityAdjustment` (- (/ 2000.0 _returnvalue_3) 1.0))))
          (bind _returnvalue_4 (+ (`local.PriorityAdjustment`) (`KismetMathLibrary.Dot_VectorVector` (`local.DirectionVector`) (`KismetMathLibrary.Normal` _returnvalue_2))))
          (if (and (< _returnvalue_3 (`local.TargetingRange`)) (> _returnvalue_4 (`local.TargetPrority`)))
            (set `local.TargetPrority` _returnvalue_4)
            (set `local.TempTargetEnemy` null)))))
    (set `local.PreviousDirectionInput` _returnvalue)
    (`/Engine/EditorBlueprintResources/StandardMacros.IsValid` _temptargetenemy
      (:`Is Valid`
        (`self.SetTarget` _temptargetenemy))
      (:`Is Not Valid`
        (`self.SetTarget` _temptargetenemy)))))

(fn `Targetting`
  (returns (`Target Actor` :type "Actor Object Reference") (Successful :type Boolean))
  (locals (TargetActor :type "Actor Object Reference") (FoundTarget :type Boolean) (ShowDebugLines :type "EDrawDebugTrace Enum" :default "ForDuration"))
  (bind _returnvalue (`self.K2_GetActorLocation`))
  (bind _array (`|MakeArray` "ObjectTypeQuery8" :!type "EObjectTypeQuery Enum"))
  (bind _showdebuglines (`local.ShowDebugLines`))
  (bind _returnvalue_2 (`SceneComponent.GetForwardVector` (`self.FollowCamera`)))
  (bind _returnvalue_3 (+ _returnvalue (* _returnvalue_2 5000.0)))
  (bind _returnvalue_4 (+ _returnvalue (* _returnvalue_2 500.0)))
  (bind (_outhits _returnvalue_5) (`KismetSystemLibrary.SphereTraceMultiForObjects` :`Start` _returnvalue_4 :`End` _returnvalue_3 :`Radius` 10.0 :`ObjectTypes` _array :`DrawDebugType` _showdebuglines :`DrawTime` 1.0))
  (if _returnvalue_5
    (for _array_element _outhits
      (bind (_bblockinghit _binitialoverlap _time _distance _location _impactpoint _normal _impactnormal _physmat _hitactor) (`GameplayStatics.BreakHitResult` _array_element))
      (bind _returnvalue_6 (message `GameplayTagAssetInterface.HasMatchingGameplayTag` _hitactor (struct :`TagName` "Team.BadGuy")))
      (if _returnvalue_6
        (set `local.TargetActor` _hitactor)
        (set `local.FoundTarget` true)
        (break)))
    (if (`local.FoundTarget`)
      (return (`local.TargetActor`) (`local.FoundTarget`))
      (else
        (bind (_outhits_2 _returnvalue_7) (`KismetSystemLibrary.SphereTraceMultiForObjects` :`Start` _returnvalue_4 :`End` _returnvalue_3 :`Radius` 200.0 :`ObjectTypes` _array :`DrawDebugType` _showdebuglines :`DrawTime` 1.0 :!label _label))
        (if _returnvalue_7
          (for _array_element_2 _outhits_2
            (bind (_bblockinghit_2 _binitialoverlap_2 _time_2 _distance_2 _location_2 _impactpoint_2 _normal_2 _impactnormal_2 _physmat_2 _hitactor_2) (`GameplayStatics.BreakHitResult` _array_element_2))
            (bind _returnvalue_8 (message `GameplayTagAssetInterface.HasMatchingGameplayTag` _hitactor_2 (struct :`TagName` "Team.BadGuy")))
            (if _returnvalue_8
              (set `local.TargetActor` _hitactor_2)
              (set `local.FoundTarget` true)
              (break)))
          (if (`local.FoundTarget`)
            (return (`local.TargetActor`) (`local.FoundTarget`))
            (else
              (bind (_outhits_3 _returnvalue_9) (`KismetSystemLibrary.SphereTraceMultiForObjects` :`Start` _returnvalue_4 :`End` _returnvalue_3 :`Radius` 200.0 :`ObjectTypes` _array :`DrawDebugType` _showdebuglines :`DrawTime` 1.0 :!label _label_2))
              (if _returnvalue_9
                (for _array_element_3 _outhits_3
                  (bind (_bblockinghit_3 _binitialoverlap_3 _time_3 _distance_3 _location_3 _impactpoint_3 _normal_3 _impactnormal_3 _physmat_3 _hitactor_3) (`GameplayStatics.BreakHitResult` _array_element_3))
                  (bind _returnvalue_10 (message `GameplayTagAssetInterface.HasMatchingGameplayTag` _hitactor_3 (struct :`TagName` "Team.BadGuy")))
                  (if _returnvalue_10
                    (set `local.TargetActor` _hitactor_3)
                    (set `local.FoundTarget` true)
                    (break)))
                (if (`local.FoundTarget`)
                  (return (`local.TargetActor`) (`local.FoundTarget`)))
                (else
                  (bind (_outhits_4 _returnvalue_11) (`KismetSystemLibrary.SphereTraceMultiForObjects` :`Start` _returnvalue_4 :`End` _returnvalue_3 :`Radius` 400.0 :`ObjectTypes` _array :`DrawTime` 1.0))
                  (if _returnvalue_11
                    (for _array_element_4 _outhits_4
                      (bind (_bblockinghit_4 _binitialoverlap_4 _time_4 _distance_4 _location_4 _impactpoint_4 _normal_4 _impactnormal_4 _physmat_4 _hitactor_4) (`GameplayStatics.BreakHitResult` _array_element_4))
                      (bind _returnvalue_12 (message `GameplayTagAssetInterface.HasMatchingGameplayTag` _hitactor_4 (struct :`TagName` "Team.BadGuy")))
                      (if _returnvalue_12
                        (set `local.TargetActor` _hitactor_4)
                        (set `local.FoundTarget` true)
                        (break))))
                  (return (`local.TargetActor`) (`local.FoundTarget`))))))
          (else
            (goto _label_2)))))
    (else
      (goto _label))))

(fn `UserConstructionScript`
  (`parent.UserConstructionScript`))