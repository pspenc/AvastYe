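; Treasure chest Blueprint that opens when damaged and awards gold once it has opened.
; GetDamaged plays the skeletal mesh animation, then after a short delay marks it opened, spawns coin and sparkle particles, and calls ChestOpened.
; Gold is a random amount between MinGold and MaxGold, added through AvastYeRGameMode, which saves the game seconds later.
; An older branch checking damage type and spawning a coin actor is disconnected.
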(event `self.ReceiveBeginPlay`
  (`parent.ReceiveBeginPlay`)
  (`PrimitiveComponent.SetCollisionEnabled` (`self.Box`) "QueryAndPhysics"))

(event `/Game/RebuildBPs/Interfaces/DamageInterface.GetDamaged`
  (params (Damage :type "Float (single-precision)") (Hitstun :type "Float (single-precision)") (ForceVector :type "Vector Structure") (`Damage Type` :type "/Game/RebuildBPs/Enumerations/DamageType Enum" :default "NewEnumerator0") (`Attack Type` :type "/Game/RebuildBPs/Enumerations/AttackType Enum" :default "NewEnumerator0") (Attacker :type "/Game/RebuildBPs/BaseCharacterRBP Object Reference") (`Hit Component` :type "PrimitiveComponent Object Reference") (`Enemy Team` :type "GameplayTag Structure") (`Status Effect` :type "/Game/RebuildBPs/StatusEffects/BaseStatusEffect Class Reference"))
  (bind _returnvalue (+ (`self.K2_GetActorLocation`) (0.0 0.0 75.0)))
  (if (not (`self.isOpened`))
    (`SkeletalMeshComponent.PlayAnimation` (`self.SkeletalMesh`) "/Game/Assets/Props/Chest/ChestTestANim.ChestTestANim" false)
    (`KismetSystemLibrary.Delay` 0.2)
    (set `self.isOpened` true)
    (bind _returnvalue_2 (`GameplayStatics.SpawnEmitterAtLocation` "/Game/Assets/VisualEffects/CoinEmitter/CoinMeshParticle.CoinMeshParticle" _returnvalue))
    (set `self.CoinEmitterReference` _returnvalue_2)
    (bind _asavast_ye_rgame_mode (cast `/Game/RebuildBPs/AvastYeRGameMode` (`GameplayStatics.GetGameMode`)))
    (`/Game/RebuildBPs/AvastYeRGameMode.CoinGather` _asavast_ye_rgame_mode (0.0 0.0))
    (`/Game/RebuildBPs/AvastYeRGameMode.IncrementGoldCount` _asavast_ye_rgame_mode (`KismetMathLibrary.RandomIntegerInRange` (`self.MinGold`) (`self.MaxGold`)))
    (`GameplayStatics.SpawnEmitterAtLocation` "/Game/Assets/VisualEffects/CamilleTestFolder/P_Sparkles.P_Sparkles" _returnvalue)
    (`self.ChestOpened`)
    (`KismetSystemLibrary.Delay` 3.0)
    (`/Game/RebuildBPs/AvastYeRGameMode.SaveGame` _asavast_ye_rgame_mode)))

(fn `UserConstructionScript`
  (`parent.UserConstructionScript`))