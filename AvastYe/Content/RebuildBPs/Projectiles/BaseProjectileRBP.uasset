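; Base projectile Blueprint that damages overlapped actors tagged as its owner's enemy team.
; On BeginPlay it applies its Stats struct when an owner name is set, otherwise loading by DisplayName from a GameInstance cache, falling back to a data table and caching the row.
; Hits send damage, radial knockback and status effect, play impact effects, and optionally destroy the projectile.
; AssignStatsFromStruct cross-assigns Knockback and ExplosiveRadius.
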(event `self.ReceiveBeginPlay`
  (if (!= (`self.CharacterOwnerName`) "None")
    (`self.AssignStatsFromStruct` (`self.Stats`))
    (else
      (`self.DrawFromDataTable`))))

(event `self.CollisionMesh.OnComponentBeginOverlap`
  (params (OverlappedComponent :type "PrimitiveComponent Object Reference") (OtherActor :type "Actor Object Reference") (OtherComp :type "PrimitiveComponent Object Reference") (OtherBodyIndex :type Integer) (bFromSweep :type Boolean) (SweepResult :type "HitResult Structure (by ref)"))
  (bind _projectileowner (`self.ProjectileOwner`))
  (bind _returnvalue (message `GameplayTagAssetInterface.HasMatchingGameplayTag` OtherActor (`/Game/RebuildBPs/BaseCharacterRBP.Enemy Team` (`self.ProjectileOwner`))))
  (if _returnvalue
    (message `/Game/RebuildBPs/Interfaces/DamageInterface.GetDamaged` OtherActor (`self.Damage`) (`self.Hitstun`) (`/Game/RebuildBPs/FunctionMacroLibraries/AvastYeActorMacros.RadialKnockbackUsingVectors` (`self.K2_GetActorLocation` OtherActor) (`self.K2_GetActorLocation`) (`self.Knockback`) (`self.Knockup`)) (`self.Damage Type`) (`self.Attack Type`) _projectileowner OtherComp (`/Game/RebuildBPs/BaseCharacterRBP.Enemy Team` _projectileowner) (`self.Status Effect`))
    (`self.PlayImpactSound`)
    (`self.PlayImpactParticles`)
    (`self.PlayImpactNiagara`)
    (if (`self.Destroy After Hit`)
      (`self.K2_DestroyActor`))))

(event `PlayImpactSound`
  (`GameplayStatics.PlaySoundAtLocation` (`self.Sound Effect`) (`self.K2_GetActorLocation`) (struct) (`self.SoundFX Volume`) (+ (`KismetMathLibrary.RandomFloatInRange` -0.1 0.1) (`self.SoundFX Pitch`)) 0.0 null null null))

(event `PlayImpactParticles`
  (`GameplayStatics.SpawnEmitterAtLocation` (`self.Impact Particle System`) (`self.K2_GetActorLocation`) (`self.K2_GetActorRotation`) (* (`KismetMathLibrary.MakeVector` 1.0 1.0 1.0) (`self.ParticleScale`))))

(event `PlayImpactNiagara`
  (`NiagaraFunctionLibrary.SpawnSystemAtLocation` (`self.Impact Niagra System`) (`self.K2_GetActorLocation`) (`self.K2_GetActorRotation`)))

(fn `AssignStatsFromStruct`
  (params (ProjStats :type "/Game/RebuildBPs/Structs/ProjStats Structure (by ref)"))
  (bind (_name _damage _hitstun _knockup _knockback _explosive _explosiveradius _damagetype _statuseffect) (break `/Game/RebuildBPs/Structs/ProjStats` ProjStats))
  (set `self.Damage` _damage)
  (set `self.Hitstun` _hitstun)
  (set `self.Knockup` _knockup)
  (set `self.ExplosiveRadius` _knockback)
  (set `self.Knockback` _explosiveradius)
  (set `self.Damage Type` _damagetype)
  (set `self.Status Effect` _statuseffect))

(fn `DrawFromDataTable`
  (bind _displayname (`self.DisplayName`))
  (bind (_data _data_found) (message `/Game/RebuildBPs/Interfaces/GameInstanceInterface.GetPreLoadedProjectileData` (`GameplayStatics.GetGameInstance`) _displayname))
  (if _data_found
    (`self.AssignStatsFromStruct` _data)
    (`KismetSystemLibrary.PrintString` (`KismetStringLibrary.Concat_StrStr` (`KismetStringLibrary.Conv_NameToString` (`self.DisplayName`)) "  Already Loaded") false)
    (else
      (bind _returnvalue (`|GetDataTableRow` "/Game/RebuildBPs/NewProjectileStatsTable.NewProjectileStatsTable" _displayname)
        (:`then`
          (`KismetSystemLibrary.PrintString` (`KismetStringLibrary.Concat_StrStr` (`KismetStringLibrary.Conv_NameToString` _displayname) "  DATA FOUND") false)
          (`self.AssignStatsFromStruct` _returnvalue)
          (message `/Game/RebuildBPs/Interfaces/GameInstanceInterface.StoreLoadedProjectileData` (`GameplayStatics.GetGameInstance`) (`self.DisplayName`) _returnvalue))
        (:`RowNotFound`
          (if (`KismetStringLibrary.NotEqual_StrStr` (`KismetStringLibrary.Conv_NameToString` _displayname) "Null")
            (`KismetSystemLibrary.PrintString` (`KismetStringLibrary.Concat_StrStr` (`KismetStringLibrary.Conv_NameToString` _displayname) " DATA NOT FOUND") false)))))))

(fn `UserConstructionScript`)