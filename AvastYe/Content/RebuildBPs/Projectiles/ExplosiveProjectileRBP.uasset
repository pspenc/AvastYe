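; Explosive projectile that detonates once when its sphere overlaps or hits something, if ExplodeOnHit is set.
; Explode plays impact sound, particle and Niagara effects, then sphere-traces for objects within ExplosionRadius, with debug drawing left on.
; Each hit actor receives a damage message carrying radial knockback, hitstun, an OnFire status and the owner's team information.
; The projectile destroys itself shortly after exploding.
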(event `self.Sphere.OnComponentBeginOverlap`
  (params (OverlappedComponent :type "PrimitiveComponent Object Reference") (OtherActor :type "Actor Object Reference") (OtherComp :type "PrimitiveComponent Object Reference") (OtherBodyIndex :type Integer) (bFromSweep :type Boolean) (SweepResult :type "HitResult Structure (by ref)"))
  (if (`self.ExplodeOnHit`)
    (`self.Explode!`)))

(event `self.Sphere.OnComponentHit`
  (params (HitComponent :type "PrimitiveComponent Object Reference") (OtherActor :type "Actor Object Reference") (OtherComp :type "PrimitiveComponent Object Reference") (NormalImpulse :type "Vector Structure") (Hit :type "HitResult Structure (by ref)"))
  (if (`self.ExplodeOnHit`)
    (`self.Explode!`)))

(event `Explode!`
  (bind _returnvalue (`self.K2_GetActorLocation`))
  (bind _projectileowner (`self.ProjectileOwner`))
  (if (not (`self.alreadyExploded`))
    (set `self.alreadyExploded` true)
    (`self.PlayImpactSound`)
    (`self.PlayImpactParticles`)
    (`self.PlayImpactNiagara`)
    (bind (_outhits _returnvalue_2) (`KismetSystemLibrary.SphereTraceMultiForObjects` :`Start` _returnvalue :`End` _returnvalue :`Radius` (`self.Explosion Radius`) :`ObjectTypes` (`|MakeArray` "ObjectTypeQuery8" "ObjectTypeQuery7" "ObjectTypeQuery11" :!type "EObjectTypeQuery Enum") :`DrawDebugType` "ForDuration" :`DrawTime` 10.0))
    (if _returnvalue_2
      (for _array_element _outhits
        (bind (_bblockinghit _binitialoverlap _time _distance _location _impactpoint _normal _impactnormal _physmat _hitactor _hitcomponent) (`GameplayStatics.BreakHitResult` _array_element))
        (message `/Game/RebuildBPs/Interfaces/DamageInterface.GetDamaged` _hitactor (`self.Damage`) (`self.Hitstun`) (`/Game/BPs/MacroFunctionLibraries/AvastYeActorMacros.RadialKnockback` _hitactor self (`self.Knockback`) (`self.Knockup`)) (`self.Damage Type`) "NewEnumerator2" _projectileowner _hitcomponent (`/Game/RebuildBPs/BaseCharacterRBP.Enemy Team` _projectileowner) "/Game/RebuildBPs/StatusEffects/OnFire.OnFire_C")
        (`/Engine/EditorBlueprintResources/StandardMacros.IsValid` _hitactor
          (:`Is Valid`
            (`/Engine/EditorBlueprintResources/StandardMacros.DoOnce` false
              (:`Completed`
                (set `self.Hit Actor` true)))))))
    (`KismetSystemLibrary.Delay` 0.2)
    (`self.PostExplode`)))

(event `PostExplode`
  (`self.K2_DestroyActor`))

(event `PlayImpactSound`
  (`GameplayStatics.PlaySoundAtLocation` (`self.Sound Effect`) (`self.K2_GetActorLocation`) (struct) 1.0 1.0 0.0 null null null))

(event `PlayImpactParticles`
  (`GameplayStatics.SpawnEmitterAtLocation` (`self.Impact Particle System`) (`self.K2_GetActorLocation`) (`self.K2_GetActorRotation`) (* (`KismetMathLibrary.MakeVector` 1.0 1.0 1.0) (`self.ParticleScale`))))

(event `PlayImpactNiagara`
  (`NiagaraFunctionLibrary.SpawnSystemAtLocation` (`self.Impact Niagra System`) (`self.K2_GetActorLocation`) (`self.K2_GetActorRotation`)))

(fn `UserConstructionScript`
  (`parent.UserConstructionScript`))