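; Base melee weapon that damages enemy-team or puzzle-tagged actors during its owner's attacks.
; BeginPlay optionally loads stats by display name from a data table, as the GameInstance decides.
; Collision overlaps, deduplicated until cleared, and an InitialAttackTrace of existing overlaps feed Damage, which sends light, heavy or special stats via GetDamagedMessage and plays impact effects.
; SpecialAttackAdditionalLogic is an empty hook, fired on the first special hit after each clear.
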(event `self.ReceiveBeginPlay`
  (`parent.ReceiveBeginPlay`)
  (bind _result (message `/Game/RebuildBPs/Interfaces/GameInstanceInterface.UseMeleeWeaponDataTable` (`GameplayStatics.GetGameInstance`)))
  (if _result
    (`self.DrawFromDataTable`))
  (`KismetSystemLibrary.Delay` 0.2)
  (set `self.FullyInit` true))

(event `self.WeaponCollision.OnComponentBeginOverlap`
  (params (OverlappedComponent :type "PrimitiveComponent Object Reference") (OtherActor :type "Actor Object Reference") (OtherComp :type "PrimitiveComponent Object Reference") (OtherBodyIndex :type Integer) (bFromSweep :type Boolean) (SweepResult :type "HitResult Structure (by ref)"))
  (bind _weaponowner (`self.WeaponOwner`))
  (`/Engine/EditorBlueprintResources/StandardMacros.IsValid` _weaponowner
    (:`Is Valid`
      (if (`/Game/RebuildBPs/BaseCharacterRBP.Attacking` _weaponowner)
        (bind _returnvalue (message `GameplayTagAssetInterface.HasMatchingGameplayTag` OtherActor (`/Game/RebuildBPs/BaseCharacterRBP.Enemy Team` (`self.WeaponOwner`))))
        (bind _returnvalue_2 (message `GameplayTagAssetInterface.HasMatchingGameplayTag` OtherActor (struct :`TagName` "PuzzleType")))
        (if (or _returnvalue_2 _returnvalue)
          (if (== (`KismetArrayLibrary.Array_Find` (`self.CharactersAlreadyHit`) OtherActor) -1)
            (`KismetArrayLibrary.Array_Add` (`self.CharactersAlreadyHit`) OtherActor)
            (`self.Damage` OtherActor OverlappedComponent (`SceneComponent.K2_GetComponentLocation` OtherComp))))))))

(event `ClearHitActorsArray`
  (`KismetArrayLibrary.Array_Clear` (`self.CharactersAlreadyHit`))
  (set `self.SpecialHit` false))

(event `Damage`
  (params (`Hit Character` :type "Actor Object Reference") (`Hit Component` :type "PrimitiveComponent Object Reference") (`Impact Location` :type "Vector Structure"))
  (bind (_specialdamage _specialhitstun _forcevector _specialdamagetype _weaponowner _team _status_effect) (`self.GetSpecialAttackStats` `Hit Character` `Impact Location`))
  (bind (_heavydamage _heavyhitstun _forcevector_2 _heavydamagetype _weaponowner_2 _team_2 _status_effect_2) (`self.GetHeavyAttackStats` `Hit Character` `Impact Location`))
  (bind (_basicdamage _basichitstun _forcevector_3 _basicdamagetype _weaponowner_3 _team_3 _status_effect_3) (`self.GetLightAttackStats` `Impact Location` `Hit Character`))
  (bind _heavy_sound_effect (`self.Heavy Sound Effect`))
  (bind _basic_sound_effect (`self.Basic Sound Effect`))
  (bind _weaponowner_4 (`self.WeaponOwner`))
  (bind _returnvalue (`self.K2_GetActorRotation` (`self.WeaponOwner`)))
  (`/Engine/EditorBlueprintResources/StandardMacros.IsValid` `Hit Character`
    (:`Is Valid`
      (if (`/Game/RebuildBPs/BaseCharacterRBP.SpecialAttacking` _weaponowner_4)
        (message `/Game/RebuildBPs/Interfaces/DamageInterface.GetDamaged` `Hit Character` _specialdamage _specialhitstun _forcevector _specialdamagetype "NewEnumerator0" _weaponowner null _team _status_effect)
        (if (not (`self.SpecialHit`))
          (set `self.SpecialHit` true)
          (`self.SpecialAttackAdditionalLogic` `Hit Character`))
        (`GameplayStatics.PlaySoundAtLocation` (`|GetArrayItem` _heavy_sound_effect (`KismetMathLibrary.RandomIntegerInRange` 0 (`KismetArrayLibrary.Array_Length` _heavy_sound_effect))) `Impact Location` (struct) 1.0 1.0 0.0 null null null :!label _label)
        (`GameplayStatics.SpawnEmitterAtLocation` (`self.Heavy Hit Particle`) `Impact Location` _returnvalue (1.25 1.25 1.25))
        (`NiagaraFunctionLibrary.SpawnSystemAtLocation` (`self.Heavy Hit Niagra System`) `Impact Location` _returnvalue)
        (elif (`/Game/RebuildBPs/BaseCharacterRBP.HeavyAttacking` _weaponowner_4)
          (message `/Game/RebuildBPs/Interfaces/DamageInterface.GetDamaged` `Hit Character` _heavydamage _heavyhitstun _forcevector_2 _heavydamagetype "NewEnumerator0" _weaponowner_2 `Hit Component` _team_2 _status_effect_2)
          (goto _label)
          (else
            (message `/Game/RebuildBPs/Interfaces/DamageInterface.GetDamaged` `Hit Character` _basicdamage _basichitstun _forcevector_3 _basicdamagetype "NewEnumerator0" _weaponowner_3 `Hit Component` _team_3 _status_effect_3)
            (`GameplayStatics.PlaySoundAtLocation` (`|GetArrayItem` _basic_sound_effect (`KismetMathLibrary.RandomIntegerInRange` 0 (`KismetArrayLibrary.Array_Length` _basic_sound_effect))) `Impact Location` (struct) 1.0 1.0 0.0 null null null)
            (`GameplayStatics.SpawnEmitterAtLocation` (`self.Basic Hit Particle`) `Impact Location` _returnvalue (0.8 0.8 0.8))
            (`NiagaraFunctionLibrary.SpawnSystemAtLocation` (`self.Basic Hit Niagra System`) `Impact Location` _returnvalue)))))))

(event `InitialAttackTrace`
  (for _array_element (`PrimitiveComponent.GetOverlappingActors` (`self.WeaponCollision`) "/Script/Engine.Actor")
    (bind _returnvalue (message `GameplayTagAssetInterface.HasMatchingGameplayTag` _array_element (`/Game/RebuildBPs/BaseCharacterRBP.Enemy Team` (`self.WeaponOwner`))))
    (bind _returnvalue_2 (message `GameplayTagAssetInterface.HasMatchingGameplayTag` _array_element (struct :`TagName` "PuzzleType")))
    (if (or _returnvalue_2 _returnvalue)
      (`self.Damage` _array_element null (`self.K2_GetActorLocation` _array_element))
      (`KismetArrayLibrary.Array_Add` (`self.CharactersAlreadyHit`) _array_element))))

(event `SpecialAttackAdditionalLogic`
  (params (ActorHit :type "Actor Object Reference")))

(fn `DrawFromDataTable`
  (bind _weapondisplayname (`self.WeaponDisplayName`))
  (bind _returnvalue (`|GetDataTableRow` "/Game/RebuildBPs/MeleeWeaponStats.MeleeWeaponStats" (`KismetStringLibrary.Conv_StringToName` _weapondisplayname))
    (:`then`
      (`KismetSystemLibrary.PrintString` (`KismetStringLibrary.Concat_StrStr` _weapondisplayname " DATA  FOUND") false)
      (bind (_weaponrange _baseattackspeed _basicdamage _basichitstun _basicknockup _basicknockback _heavydamage _heavyhitstun _heavyknockup _heavyknockback _specialdamage _specialhitstun _specialknockup _specialknockback) (break `/Game/RebuildBPs/Weapons/WeaponStatContainers/MeleeWeaponStatStruct` _returnvalue))
      (set `self.Range` _weaponrange)
      (set `self.Attack Speed` _baseattackspeed)
      (set `self.Basic Damage` _basicdamage)
      (set `self.Basic Hitstun` _basichitstun)
      (set `self.Basic Knockup` _basicknockup)
      (set `self.Basic Knockback` _basicknockback)
      (set `self.Heavy Damage` _heavydamage)
      (set `self.Heavy Knockback` _heavyknockback)
      (set `self.Heavy Knockup` _heavyknockup)
      (set `self.Special Knockup` _specialknockup)
      (set `self.Special Damage` _specialdamage)
      (set `self.Special Knockback` _specialknockback)
      (set `self.Heavy Hitstun` _heavyhitstun)
      (set `self.Special Hitstun` _specialhitstun))
    (:`RowNotFound`
      (`KismetSystemLibrary.PrintString` (`KismetStringLibrary.Concat_StrStr` _weapondisplayname " DATA NOT FOUND") false))))

(fn `UserConstructionScript`
  (`parent.UserConstructionScript`))