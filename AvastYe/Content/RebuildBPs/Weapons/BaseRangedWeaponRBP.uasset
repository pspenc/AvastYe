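; Base ranged weapon actor that fires projectiles at a target actor with muzzle flash and sound.
; On BeginPlay it takes fire rate, projectile class and projectile stats from the GameInstance cache, falling back to the owning character's data table row and caching that result.
; Shoot spawns one aimed projectile with those stats, while Blunderbuss spawns a burst of separate pellet projectiles with random pitch and yaw spread.
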(event `self.ReceiveBeginPlay`
  (`parent.ReceiveBeginPlay`)
  (`self.DrawFromDataTable`))

(event `Shoot`
  (params (`Target Actor` :type "Actor Object Reference") (`Target Location` :type "Vector Structure"))
  (bind _returnvalue (`SceneComponent.K2_GetComponentLocation` (`self.Projectile Spawn`)))
  (`/Engine/EditorBlueprintResources/StandardMacros.IsValid` `Target Actor`
    (:`Is Valid`
      (`self.PlayFX` `Target Actor`)
      (`|SpawnActorFromClass` (`self.Projectile Class`) (`KismetMathLibrary.MakeTransform` _returnvalue (`KismetMathLibrary.FindLookAtRotation` _returnvalue (`self.K2_GetActorLocation` `Target Actor`))) "Undefined" "OverrideRootScale" null (`self.WeaponOwner`) (`self.ProjectileStats`) `Target Actor` null)
      (`GameplayStatics.PlaySoundAtLocation` (`self.ShootSoundEffect`) (`self.K2_GetActorLocation`) (struct) 1.0 1.0 0.0 null null null))))

(event `Blunderbuss`
  (params (TargetActor :type "Actor Object Reference"))
  (bind _returnvalue (`SceneComponent.K2_GetComponentLocation` (`self.Projectile Spawn`)))
  (`/Engine/EditorBlueprintResources/StandardMacros.IsValid` TargetActor
    (:`Is Valid`
      (`self.PlayFX` TargetActor)
      (`GameplayStatics.PlaySoundAtLocation` (`self.ShootSoundEffect`) _returnvalue (struct) 2.0 0.5 0.0 null null null)
      (for _ (range 21)
        (bind _newtransform (`self.BulletSpread` 15.0 (`KismetMathLibrary.MakeTransform` _returnvalue (`KismetMathLibrary.FindLookAtRotation` _returnvalue (`self.K2_GetActorLocation` TargetActor)))))
        (`|SpawnActorFromClass` "/Game/RebuildBPs/Projectiles/BlunderbussProjectile.BlunderbussProjectile_C" _newtransform "Undefined" "OverrideRootScale" null (`self.WeaponOwner`) (struct) null null)))))

(event `PlayFX`
  (params (Target :type "Actor Object Reference"))
  (bind _returnvalue (`SceneComponent.K2_GetComponentLocation` (`self.Projectile Spawn`)))
  (`GameplayStatics.SpawnEmitterAtLocation` (`self.MuzzleFlashFX`) _returnvalue (`KismetMathLibrary.FindLookAtRotation` _returnvalue (`self.K2_GetActorLocation` Target))))

(fn `AssignStatsFromStruct`
  (params (NewRangedWeaponStruct :type "/Game/RebuildBPs/Structs/NewRangedWeaponStruct Structure (by ref)"))
  (bind (_name _firerate _standardshotprojectile _standardshotclassreference) (break `/Game/RebuildBPs/Structs/NewRangedWeaponStruct` NewRangedWeaponStruct))
  (set `self.FireRate` _firerate)
  (set `self.Projectile Class` _standardshotclassreference)
  (set `self.ProjectileStats` _standardshotprojectile))

(fn `BulletSpread`
  (params (Spread :type "Float (double-precision)") (InTransform :type "Transform Structure"))
  (returns (NewTransform :type "Transform Structure"))
  (bind _returnvalue (* Spread -1.0))
  (return (`KismetMathLibrary.MakeTransform` (.location InTransform) (`KismetMathLibrary.MakeRotator` (.roll (.rotation InTransform)) (+ (.pitch (.rotation InTransform)) (`KismetMathLibrary.RandomFloatInRange` _returnvalue Spread)) (+ (.yaw (.rotation InTransform)) (`KismetMathLibrary.RandomFloatInRange` _returnvalue Spread))) (.scale InTransform))))

(fn `DrawFromDataTable`
  (bind _characterownername (`self.CharacterOwnerName`))
  (bind _weapondisplayname (`self.WeaponDisplayName`))
  (bind (_data _data_found) (message `/Game/RebuildBPs/Interfaces/GameInstanceInterface.GetPreLoadedRangedWeaponData` (`GameplayStatics.GetGameInstance`) _weapondisplayname))
  (if _data_found
    (`self.AssignStatsFromStruct` _data)
    (`KismetSystemLibrary.PrintString` (`KismetStringLibrary.Concat_StrStr` (`KismetStringLibrary.Conv_NameToString` (`self.WeaponDisplayName`)) "  Already Loaded") false)
    (elif (!= _characterownername "None")
      (bind _returnvalue (`|GetDataTableRow` "/Game/RebuildBPs/CharacterDataTable.CharacterDataTable" _characterownername)
        (:`then`
          (`KismetSystemLibrary.PrintString` (`KismetStringLibrary.Concat_StrStr` (`KismetStringLibrary.Conv_NameToString` _weapondisplayname) " DATA  FOUND") false)
          (bind (_basicstats _meleeweapon _rangedweapon) (break `/Game/RebuildBPs/Structs/NewCharacterStruct` _returnvalue))
          (`self.AssignStatsFromStruct` _rangedweapon)
          (message `/Game/RebuildBPs/Interfaces/GameInstanceInterface.StoreLoadedRangedWeaponData` (`GameplayStatics.GetGameInstance`) (`self.WeaponDisplayName`) _rangedweapon))
        (:`RowNotFound`
          (`KismetSystemLibrary.PrintString` (`KismetStringLibrary.Concat_StrStr` (`KismetStringLibrary.Conv_NameToString` _weapondisplayname) " DATA NOT FOUND") false :!label _label)))
      (else
        (goto _label)))))

(fn `UserConstructionScript`
  (`parent.UserConstructionScript`))