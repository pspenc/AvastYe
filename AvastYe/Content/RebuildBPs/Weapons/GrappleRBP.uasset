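; GrappleRBP is a work-in-progress grapple weapon Blueprint that stores an origin and target when Grapple fires.
; Grapple starts a fast looping timer on GrappleLoop, which so far only prints debug text; GrappleReleased clears it.
; SendGrapple shows GrappleLine and interpolates it toward a valid target until within range, releasing if the target is invalid.
; Nothing in this Blueprint calls SendGrapple.
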(event `Grapple`
  (params (Origin :type "ChildActorComponent Object Reference") (GrappleTarget :type "Actor Object Reference"))
  (set `self.Origin` Origin)
  (set `self.GrappleTarget` GrappleTarget)
  (`KismetSystemLibrary.K2_SetTimer` null "GrappleLoop" 0.01 true) ; Enter Grapple Loop
)

(event `Grapple Released`
  (`KismetSystemLibrary.K2_ClearTimer` null "GrappleLoop")
  (`KismetSystemLibrary.PrintString` "Released" true true (struct :`R` 1.0 :`B` 0.028928 :`A` 1.0)))

(fn `GrappleLoop`
  (`KismetSystemLibrary.PrintString` "Grapple" true true (struct :`R` 0.031705 :`G` 1.0 :`A` 1.0)))

(fn `SendGrapple`
  (bind _grappleline (`self.GrappleLine`))
  (bind _grappletarget (`self.GrappleTarget`))
  (bind _returnvalue (`SceneComponent.K2_GetComponentLocation` _grappleline))
  (bind _returnvalue_2 (`self.K2_GetActorLocation` _grappletarget))
  (`/Engine/EditorBlueprintResources/StandardMacros.IsValid` _grappletarget
    (:`Is Valid`
      (`SceneComponent.SetVisibility` _grappleline true true) ; Make the Grapple Visible
      (if (not (<= (`KismetMathLibrary.VSize` (- _returnvalue _returnvalue_2)) 100.0))
        (`SceneComponent.K2_SetWorldLocation` (`self.GrappleLine`) (`KismetMathLibrary.VInterpTo` _returnvalue _returnvalue_2 (`GameplayStatics.GetWorldDeltaSeconds`) 10.0) false false)))
    (:`Is Not Valid`
      (`self.Grapple Released`))))

(fn `UserConstructionScript`
  (`parent.UserConstructionScript`))